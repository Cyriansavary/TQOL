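; Base wolf AI character that hunts heroes, takes damage and dies.
; On possession it retries FindEnemy until it targets the hero with the fewest attackers, balancing via a per-hero counter, then re-issues AI MoveTo in a loop while alive.
; TakeDamage derives a hit direction and returns XP and death state; death releases the attacker slot and plays a montage, currently identical for every direction.
; StartRagdoll switches the mesh to physics with a velocity-based impulse.
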(event Custom|OnAISpawned
  (bind (_isvalidplayerfound _newenemy) (CallFunction|FindEnemy :!label _label))
  (if _isvalidplayerfound
    (CallFunction|SetTargetPlayer _newenemy)
    (CallFunction|MovetoPlayer)
    (else
      (Utilities|FlowControl|Delay 0.5)
      (goto _label))))

(event Custom|MoveToPlayer
  (if (Variables|Default|GetIsAlive)
    (bind _movementresult (AI|AIMoveTo self "0, 0, 0" (Variables|Default|GetTargetPlayer) 1e+02 false)
      (:OnSuccess
        _)
      (:OnFail
        _))
    (switch Utilities|FlowControl|Switch|SwitchonEPathFollowingResult _movementresult
      (:Success
        _)
      (:Blocked
        _)
      (:OffPath
        _)
      (:Invalid
        _))
    (Utilities|FlowControl|Delay 2.0)
    (CallFunction|MovetoPlayer)))

(event Custom|Die
  (params (DamageDirection :type E_DamageDirection%20Enum :default "NewEnumerator0"))
  (bind _targetplayer (Variables|Default|GetTargetPlayer))
  (Utilities|IsValid _targetplayer
    (:Is%20Valid
      (Math|Integer|DecrementInt (Variables|/Game/Characters/BP_Hero_Base.BP_Hero_Base_C|GetNRAiAttacker _targetplayer)
        (:%20%20
          _)))
    (:Is%20Not%20Valid
      _))
  (CallFunction|MCPlayDathMontage DamageDirection))

(event Custom|MC_PlayDathMontage
  (params (DamageDirection :type E_DamageDirection%20Enum :default "NewEnumerator0"))
  (bind _deathmontage (CallFunction|GetDeathMontage DamageDirection))
  (Animation|Montage|PlayMontage (Variables|Character|GetMesh) _deathmontage))

(event Custom|StartRagdoll
  (bind _returnvalue (Utilities|Name|MakeLiteralName "Wolf_-Pelvis"))
  (bind _mesh (Variables|Character|GetMesh))
  (bind _charactermovement (Variables|Character|GetCharacterMovement))
  (bind _returnvalue_2 (Pawn|Components|CharacterMovement|GetLastUpdateVelocity _charactermovement))
  (Collision|SetCollisionEnabled (Variables|Collision|GetCapsuleComponent) "NoCollision")
  (Collision|SetCollisionProfileName _mesh "Ragdoll" true :!class /Script/Engine.PrimitiveComponent)
  (Class|SkeletalMeshComponent|SetAllBodiesBelowSimulatePhysics _mesh _returnvalue true true)
  (Physics|AddImpulse _mesh (+ _returnvalue_2 (* (Math|Vector|Normalize _returnvalue_2) 4e+02)) _returnvalue true)
  (if (Networking|IsServer)
    (Components|Movement|StopMovementImmediately (Variables|Character|GetCharacterMovement))))

(event EventPossessed
  (params (NewController :type Controller%20Object%20Reference))
  (bind _asbp_ai_controller_base (Utilities|Casting|CastToBP_Ai_Controller_Base NewController))
  (Variables|Default|SetAs%20BP%20Ai%20Controller%20Base _asbp_ai_controller_base)
  (CallFunction|OnAISpawned))

(fn ConstructionScript)

(fn FindEnemy
  (bind _outactors (Actor|GetAllActorsOfClass "/Game/Characters/BP_Hero_Base.BP_Hero_Base_C"))
  (bind _output_get (LocalVariables|SetLcl_AllPlayer _outactors))
  (if (Utilities|Array|IsNotEmpty _output_get)
    (if (== (Utilities|Array|Length (LocalVariables|GetLcl_AllPlayer)) 1)
      (LocalVariables|SetLcl_IsValidPlayerFound true)
      (LocalVariables|SetLcl_NewEnemy (Utilities|Array|Get(acopy) (LocalVariables|GetLcl_AllPlayer)))
      (else
        (for _array_element (LocalVariables|GetLcl_AllPlayer)
          (Utilities|Array|Add (LocalVariables|GetLcl_AllAttackerNRs) (Variables|/Game/Characters/BP_Hero_Base.BP_Hero_Base_C|GetNRAiAttacker _array_element)))
        (LocalVariables|SetLcl_LowestIndex (.IndexOfMinValue (Math|Integer|MinOfIntArray (LocalVariables|GetLcl_AllAttackerNRs))))
        (if (== (LocalVariables|GetLcl_LowestIndex) -1)
          (LocalVariables|SetLcl_IsValidPlayerFound false)
          (else
            (LocalVariables|SetLcl_NewEnemy (Utilities|Array|Get(acopy) (LocalVariables|GetLcl_AllPlayer) (LocalVariables|GetLcl_LowestIndex)))
            (LocalVariables|SetLcl_IsValidPlayerFound true)))))
    (else
      (LocalVariables|SetLcl_IsValidPlayerFound false)))
  (return (LocalVariables|GetLcl_IsValidPlayerFound) (LocalVariables|GetLcl_NewEnemy)))

(fn GetDeathMontage
  (params (DamageDirection :type E_DamageDirection%20Enum :default "NewEnumerator0"))
  (switch Utilities|FlowControl|Switch|SwitchonE_DamageDirection DamageDirection
    (:NewEnumerator0
      _)
    (:NewEnumerator1
      _)
    (:NewEnumerator2
      _)
    (:NewEnumerator3
      _))
  (LocalVariables|SetLcl_DeathMonatge "/Game/AnimalVarietyPack/Wolf/Animations/ANIM_Wolf_Death_Montage.ANIM_Wolf_Death_Montage")
  (return (LocalVariables|GetLcl_DeathMonatge)))

(fn SetTargetPlayer
  (params (TargetPlayer :type BP%20Hero%20Base%20Object%20Reference))
  (Utilities|IsValid (Variables|Default|GetTargetPlayer)
    (:Is%20Valid
      (Math|Integer|DecrementInt (Variables|/Game/Characters/BP_Hero_Base.BP_Hero_Base_C|GetNRAiAttacker (Variables|Default|GetTargetPlayer))
        (:%20%20
          _)))
    (:Is%20Not%20Valid
      _))
  (bind _output_get (Variables|Default|SetTargetPlayer TargetPlayer))
  (Math|Integer|IncrementInt (Variables|/Game/Characters/BP_Hero_Base.BP_Hero_Base_C|GetNRAiAttacker _output_get)
    (:%20%20
      (Variables|/Game/AI/BP_Ai_Controller_Base.BP_Ai_Controller_Base_C|SetTargetPlayer (Variables|Default|GetAs%20BP%20Ai%20Controller%20Base) (Variables|Default|GetTargetPlayer))
      (return))))

(fn TakeDamage
  (params (Attacker :type Actor%20Object%20Reference) (Amount :type Float%20%28double-precision%29))
  (if (Variables|Default|GetIsAlive)
    (LocalVariables|SetLcl_IsValidHit true)
    (bind _output_get (LocalVariables|SetLcl_DamageYaw (Math|Rotator|NormalizeAxis (- (.yaw (Math|Rotator|MakeRotfromZ (- (Transformation|GetActorLocation Attacker) (Transformation|GetActorLocation)))) (- (.yaw (Transformation|GetActorRotation)) (.yaw (Variables|/Script/Engine.SceneComponent|GetRelativeRotation (Variables|Character|GetMesh))))))))
    (if (< _output_get 0.0)
      (if (Math|Float|InRange(Float) (LocalVariables|GetLcl_DamageYaw) -135.0 -45.0 true false)
        (LocalVariables|SetLcl_DamageDirection "NewEnumerator2")
        (elif (>= (LocalVariables|GetLcl_DamageYaw) -45.0)
          (LocalVariables|SetLcl_DamageDirection "NewEnumerator0")
          (else
            (LocalVariables|SetLcl_DamageDirection "NewEnumerator1"))))
      (elif (Math|Float|InRange(Float) (LocalVariables|GetLcl_DamageYaw) 45.0 135.0 false)
        (LocalVariables|SetLcl_DamageDirection "NewEnumerator3")
        (elif (<= (LocalVariables|GetLcl_DamageYaw) 45.0)
          (LocalVariables|SetLcl_DamageDirection "NewEnumerator0")
          (else
            (LocalVariables|SetLcl_DamageDirection "NewEnumerator1")))))
    (bind _output_get_2 (Variables|Default|SetHealth (- (Variables|Default|GetHealth) Amount)))
    (if (<= _output_get_2 0.0)
      (Variables|Default|SetIsAlive false)
      (CallFunction|Die (LocalVariables|GetLcl_DamageDirection)))
    (else
      (LocalVariables|SetLcl_IsValidHit false)))
  (return (not (Variables|Default|GetIsAlive)) (Variables|Default|GetXPWhenKilled) (LocalVariables|GetLcl_IsValidHit)))