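; Skeleton AI enemy that hunts living hero players and chases them once possessed by its AI controller.
; FindPlayer favors the hero with the fewest AI attackers, and per-player attacker counts spread enemies across targets.
; An AIMoveTo loop repeats while the target lives, then searches again.
; Death removes the attack trigger, releases the attacker slot and calls an empty GetDeathMontage hook, with a separate event for montage playback.
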(event Custom|Move%20To%20player
  (if (Variables|Default|GetIsItAlive)
    (bind _movementresult (AI|AIMoveTo self "0, 0, 0" (Variables|Default|GetTarget) 5e+01 false)
      (:OnSuccess
        _)
      (:OnFail
        _))
    (switch Utilities|FlowControl|Switch|SwitchonEPathFollowingResult _movementresult
      (:Success
        _)
      (:Blocked
        _)
      (:OffPath
        _)
      (:Invalid
        _))
    (Utilities|FlowControl|Delay 0.1)
    (bind _targetplayer (Variables|Default|GetTargetPlayer)
      (:then
        (if (Variables|/Game/Characters/BP_Hero_Base.BP_Hero_Base_C|GetIsAlive _targetplayer)
          (CallFunction|MovetoPlayer)
          (else
            (Variables|Default|SetTarget 0 :!label _label)
            (CallFunction|OnSpawned))))
      (:else
        (goto _label)))))

(event Custom|OnSpawned
  (bind (_isvalidplayerfound _newenemy) (CallFunction|FindEnemy :!label _label))
  (if _isvalidplayerfound
    (CallFunction|SetTargetPlayer _newenemy)
    (Utilities|FlowControl|Delay 0.2)
    (CallFunction|MovetoPlayer)
    (else
      (Utilities|FlowControl|Delay 0.5)
      (goto _label))))

(event Custom|Death
  (bind _target (Variables|Default|GetTarget))
  (Components|DestroyComponent (Variables|Default|GetAttackTrigger))
  (Variables|Default|SetIsAttacking false)
  (Utilities|IsValid _target
    (:Is%20Valid
      (Math|Integer|DecrementInt (Variables|/Game/Characters/BP_Hero_Base.BP_Hero_Base_C|GetNRAiAttacker _target)
        (:%20%20
          _)))
    (:Is%20Not%20Valid
      _))
  (CallFunction|GetDeathMontage))

(event Custom|MC_DeathMontage
  (params (AMToPlay :type Anim%20Montage%20Object%20Reference))
  (Animation|Montage|PlayMontage (Variables|Character|GetMesh) AMToPlay))

(event EventBeginPlay)

(event Collision|EventActorBeginOverlap
  (params (OtherActor :type Actor%20Object%20Reference)))

(event EventTick
  (params (DeltaSeconds :type Float%20%28single-precision%29))
  (|CallParentFunction DeltaSeconds) ; This node is disabled and will not be called.\nDrag off pins to build functionality.
)

(event EventPossessed
  (params (NewController :type Controller%20Object%20Reference))
  (bind _asbp_ai_controller_skeleton (Utilities|Casting|CastToBP_AI_ControllerSkeleton NewController))
  (Variables|Default|SetAs%20BP%20AI%20Controller%20Skeleton _asbp_ai_controller_skeleton)
  (CallFunction|OnSpawned)
  (Variables|Default|SetDefault%20Walk%20Speed (Variables|/Script/Engine.CharacterMovementComponent|GetMaxWalkSpeed (Variables|Character|GetCharacterMovement))))

(fn ConstructionScript
  (|CallParentFunction))

(fn FindPlayer
  ;[1 1 1] On créer une liste de joueur qu'on va cibler
  (bind _outactors (Actor|GetAllActorsOfClass "/Game/Characters/BP_Hero_Base.BP_Hero_Base_C"))
  (bind _output_get (LocalVariables|SetLcl_AllPlayers _outactors))
  (bind _arrayelement (Utilities|Array|ReverseforEachLoop _output_get)
    (:LoopBody
      ;[1 1 1] Si le joueur n'est plus en vie on le retire de la liste des cibles
      (if (not (Variables|/Game/Characters/BP_Hero_Base.BP_Hero_Base_C|GetIsAlive _arrayelement))
        (Utilities|Array|RemoveItem (LocalVariables|GetLcl_AllPlayers) _arrayelement)))
    (:Completed
      (if (Utilities|Array|IsNotEmpty (LocalVariables|GetLcl_AllPlayers))
        (if (== (Utilities|Array|Length (LocalVariables|GetLcl_AllPlayers)) 1)
          (LocalVariables|SetLcl_IsValid true)
          (LocalVariables|SetLcl_NewTarget (Utilities|Array|Get(acopy) (LocalVariables|GetLcl_AllPlayers)))
          (else
            (for _array_element (LocalVariables|GetLcl_AllPlayers)
              (Utilities|Array|Add (LocalVariables|GetLcl_AllAttackersNRs) (Variables|/Game/Characters/BP_Hero_Base.BP_Hero_Base_C|GetNRAiAttacker _array_element)))
            (LocalVariables|SetLcl_LowestIndex (.IndexOfMinValue (Math|Integer|MinOfIntArray (LocalVariables|GetLcl_AllAttackersNRs))))
            (if (== (LocalVariables|GetLcl_LowestIndex) -1)
              (LocalVariables|SetLcl_IsValid false)
              (else
                (LocalVariables|SetLcl_NewTarget (Utilities|Array|Get(acopy) (LocalVariables|GetLcl_AllPlayers) (LocalVariables|GetLcl_LowestIndex)))
                (LocalVariables|SetLcl_IsValid true)))))
        (else
          (LocalVariables|SetLcl_IsValid false)))
      (return (LocalVariables|GetLcl_IsValid) (LocalVariables|GetLcl_NewTarget)))))

(fn SetTargetPlayer
  (params (Target :type BP%20Hero%20Base%20Object%20Reference))
  (Utilities|IsValid (Variables|Default|GetTarget)
    (:Is%20Valid
      (Math|Integer|DecrementInt (Variables|/Game/Characters/BP_Hero_Base.BP_Hero_Base_C|GetNRAiAttacker (Variables|Default|GetTarget))
        (:%20%20
          _)))
    (:Is%20Not%20Valid
      _))
  (bind _output_get (Variables|Default|SetTarget Target))
  (Math|Integer|IncrementInt (Variables|/Game/Characters/BP_Hero_Base.BP_Hero_Base_C|GetNRAiAttacker _output_get)
    (:%20%20
      (Variables|/Game/AI/Wolf/BP_Ai_Controller_Base.BP_Ai_Controller_Base_C|SetTargetPlayer (Variables|Default|GetAs%20BP%20Ai%20Controller%20Base) (Variables|Default|GetTargetPlayer)))))

(fn GetDeathMontage)