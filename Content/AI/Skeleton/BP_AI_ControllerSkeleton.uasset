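; AI controller for the skeleton enemy that picks which hero it chases, based on sight.
; On possession it caches the skeleton pawn, then listens to AI Perception updates and handles only the sight sense.
; A newly seen hero becomes the pawn's target and triggers its move-to-player, but only while switching is allowed.
; A CanSwitch flag locks the target while it stays visible and reopens switching when sight of it is lost.
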(event OnTargetPerceptionUpdated(AIPerception)
  (params (Actor :type Actor%20Object%20Reference) (Stimulus :type AI%20Stimulus%20Structure))
  (bind _bsuccessfullysensed (Utilities|Struct|BreakAIStimulus Stimulus))
  (bind _as_bp_ai_skeleton (Variables|Default|GetAs%20BP%20AI%20Skeleton))
  (bind _returnvalue (Class|AIPerceptionSystem|GetSenseClassforStimulus Stimulus))
  (if (== _returnvalue "/Script/AIModule.AISense_Sight")
    (if (!= Actor (Variables|Default|GetTarget%20Player))
      (bind _asbp_hero_base (Utilities|Casting|CastToBP_Hero_Base Actor))
      (if _bsuccessfullysensed
        (if (Variables|Default|GetCanSwitch)
          (Variables|Default|SetCanSwitch false)
          (Default|SetTargetPlayer _as_bp_ai_skeleton _asbp_hero_base)
          (Default|MovetoPlayer _as_bp_ai_skeleton)))
      (elif _bsuccessfullysensed
        (Variables|Default|SetCanSwitch false)
        (else
          (Variables|Default|SetCanSwitch true))))))

(event EventBeginPlay
  (|CallParentFunction) ; This node is disabled and will not be called.\nDrag off pins to build functionality.
)

(event EventTick
  (params (DeltaSeconds :type Float%20%28single-precision%29))
  (|CallParentFunction DeltaSeconds) ; This node is disabled and will not be called.\nDrag off pins to build functionality.
)

(event EventPossess
  (params (PossessedPawn :type Pawn%20Object%20Reference))
  (bind _asbp_ai_skeleton (Utilities|Casting|CastToBP_AI_Skeleton PossessedPawn))
  (Variables|Default|SetAs%20BP%20AI%20Skeleton _asbp_ai_skeleton))

(fn ConstructionScript
  (|CallParentFunction))