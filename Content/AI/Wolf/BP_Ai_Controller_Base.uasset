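; Base AI controller for wolf enemies that uses AI Perception sight to pick a hero to chase.
; On possess it caches the wolf pawn, then hands a newly seen hero to it through SetTargetPlayer and MoveToPlayer.
; A CanSwitchTarget flag locks targeting after a pick and reopens only when sight of TargetPlayer is lost.
; TargetPlayer is compared here but never assigned in this graph.
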(event OnTargetPerceptionUpdated(AIPerception)
  (params (Actor :type Actor%20Object%20Reference) (Stimulus :type AI%20Stimulus%20Structure))
  (bind _bsuccessfullysensed (Utilities|Struct|BreakAIStimulus Stimulus))
  (bind _as_bp_ai_wolf_base (Variables|Default|GetAs%20BP%20AI%20Wolf%20Base))
  (bind _returnvalue (Class|AIPerceptionSystem|GetSenseClassforStimulus Stimulus))
  (if (== _returnvalue "/Script/AIModule.AISense_Sight")
    (if (!= Actor (Variables|Default|GetTargetPlayer))
      (bind _asbp_hero_base (Utilities|Casting|CastToBP_Hero_Base Actor))
      (if _bsuccessfullysensed
        (if (Variables|Default|GetCanSwitchTarget)
          (Variables|Default|SetCanSwitchTarget false)
          (Default|SetTargetPlayer _as_bp_ai_wolf_base _asbp_hero_base)
          (Default|MovetoPlayer _as_bp_ai_wolf_base)))
      (elif _bsuccessfullysensed
        (Variables|Default|SetCanSwitchTarget false)
        (else
          (Variables|Default|SetCanSwitchTarget true))))))

(event EventBeginPlay)

(event EventTick
  (params (DeltaSeconds :type Float%20%28single-precision%29)))

(event EventPossess
  (params (PossessedPawn :type Pawn%20Object%20Reference))
  (bind _asbp_ai_wolf_base (Utilities|Casting|CastToBP_AI_Wolf_Base PossessedPawn))
  (Variables|Default|SetAs%20BP%20AI%20Wolf%20Base _asbp_ai_wolf_base))

(fn ConstructionScript)