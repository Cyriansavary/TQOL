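; Base wolf enemy AI character for a multiplayer game that hunts and melees living heroes.
; On possession it targets the hero with fewest attackers and chases via a retrying AI MoveTo.
; An overlap trigger loops multicast attack montages, while a server-side head-socket sphere trace deals damage.
; TakeDamage doubles headshots and computes hit direction, though every direction plays one death montage; StartRagdoll handles physics and delayed destruction.
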(event OnComponentBeginOverlap(AttackTrigger)
  (params (OverlappedComponent :type Primitive%20Component%20Object%20Reference) (OtherActor :type Actor%20Object%20Reference) (OtherComp :type Primitive%20Component%20Object%20Reference) (OtherBodyIndex :type Integer) (bFromSweep :type Boolean) (SweepResult :type Hit%20Result%20Structure%20%28by%20ref%29))
  (if (and (== OtherActor (Variables|Default|GetTargetPlayer)) (Variables|Default|GetIsAlive))
    (Variables|Default|SetCanAttack true)
    (Variables|Default|SetAnimIndex 0)
    (Variables|/Script/Engine.CharacterMovementComponent|SetMaxWalkSpeed (Variables|Character|GetCharacterMovement) 0.0)
    (CallFunction|AttackLoop)))

(event OnComponentEndOverlap(AttackTrigger)
  (params (OverlappedComponent :type Primitive%20Component%20Object%20Reference) (OtherActor :type Actor%20Object%20Reference) (OtherComp :type Primitive%20Component%20Object%20Reference) (OtherBodyIndex :type Integer))
  (if (== OtherActor (Variables|Default|GetTargetPlayer))
    (CallFunction|MCStopCurrentMontage)
    (Variables|Default|SetCanAttack false)
    (Variables|/Script/Engine.CharacterMovementComponent|SetMaxWalkSpeed (Variables|Character|GetCharacterMovement) (Variables|Default|GetDefault%20Walk%20Speed))
    (CallFunction|OnAISpawned)))

(event Custom|OnAISpawned
  (bind (_isvalidplayerfound _newenemy) (CallFunction|FindEnemy :!label _label))
  (if _isvalidplayerfound
    (CallFunction|SetTargetPlayer _newenemy)
    (Utilities|FlowControl|Delay 0.2)
    (CallFunction|MovetoPlayer)
    (else
      (Utilities|FlowControl|Delay 0.5)
      (goto _label))))

(event Custom|MoveToPlayer
  (if (Variables|Default|GetIsAlive)
    (bind _movementresult (AI|AIMoveTo self "0, 0, 0" (Variables|Default|GetTargetPlayer) 5e+01 false)
      (:OnSuccess
        _)
      (:OnFail
        _))
    (switch Utilities|FlowControl|Switch|SwitchonEPathFollowingResult _movementresult
      (:Success
        _)
      (:Blocked
        _)
      (:OffPath
        _)
      (:Invalid
        _))
    (Utilities|FlowControl|Delay 0.1)
    (bind _targetplayer (Variables|Default|GetTargetPlayer)
      (:then
        (if (Variables|/Game/Characters/BP_Hero_Base.BP_Hero_Base_C|GetIsAlive _targetplayer)
          (CallFunction|MovetoPlayer)
          (else
            (Variables|Default|SetTargetPlayer 0 :!label _label)
            (CallFunction|OnAISpawned))))
      (:else
        (goto _label)))))

(event Custom|Die
  (params (DamageDirection :type E_DamageDirection%20Enum :default "NewEnumerator0"))
  (bind _targetplayer (Variables|Default|GetTargetPlayer))
  (Components|DestroyComponent (Variables|Default|GetAttackTrigger))
  (Variables|Default|SetCanAttack false)
  (Utilities|IsValid _targetplayer
    (:Is%20Valid
      (Math|Integer|DecrementInt (Variables|/Game/Characters/BP_Hero_Base.BP_Hero_Base_C|GetNRAiAttacker _targetplayer)
        (:%20%20
          _)))
    (:Is%20Not%20Valid
      _))
  (bind _deathmontage (CallFunction|GetDeathMontage DamageDirection))
  (CallFunction|MCPlayDeathMontage _deathmontage))

(event Custom|MC_PlayDeathMontage
  (params (MontageToPlay :type Anim%20Montage%20Object%20Reference))
  (Animation|Montage|PlayMontage (Variables|Character|GetMesh) MontageToPlay))

(event Custom|StartRagdoll
  (bind _returnvalue (Utilities|Name|MakeLiteralName "Wolf_-Pelvis"))
  (bind _mesh (Variables|Character|GetMesh))
  (bind _charactermovement (Variables|Character|GetCharacterMovement))
  (bind _returnvalue_2 (Pawn|Components|CharacterMovement|GetLastUpdateVelocity _charactermovement))
  (Collision|SetCollisionEnabled (Variables|Collision|GetCapsuleComponent) "NoCollision")
  (Collision|SetCollisionProfileName _mesh "Ragdoll" true :!class /Script/Engine.PrimitiveComponent)
  (Class|SkeletalMeshComponent|SetAllBodiesBelowSimulatePhysics _mesh _returnvalue true true)
  (Physics|AddImpulse _mesh (+ _returnvalue_2 (* (Math|Vector|Normalize _returnvalue_2) 4e+02)) _returnvalue true)
  (if (Networking|IsServer)
    (Components|Movement|StopMovementImmediately (Variables|Character|GetCharacterMovement))
    (Utilities|FlowControl|Delay (Math|Conversions|ToFloat(Integer) (Math|Random|RandomIntegerinRange 3 6)))
    (Actor|DestroyActor)))

(event Custom|MC_RemoveClientTrigger
  (if (not (Networking|IsServer))
    (Components|DestroyComponent (Variables|Default|GetAttackTrigger))
    (Actor|Tick|SetActorTickEnabled false)))

(event Custom|MC_StopCurrentMontage
  (Animation|StopAnimMontage 0))

(event Custom|AttackLoop
  (bind _targetplayer (Variables|Default|GetTargetPlayer)
    (:then
      (if (Variables|/Game/Characters/BP_Hero_Base.BP_Hero_Base_C|GetIsAlive _targetplayer)
        (if (and (Variables|Default|GetIsAlive) (Variables|Default|GetCanAttack))
          (CallFunction|MCPlayAttackMontage (Utilities|Array|Get(acopy) (Variables|Default|GetAllAttackAnim) (Variables|Default|GetAnimIndex))))
        (else
          (Variables|Default|SetCanAttack false :!label _label)
          (Variables|/Game/AI/Wolf/BP_Ai_Controller_Base.BP_Ai_Controller_Base_C|SetCanSwitchTarget (Variables|Default|GetAs%20BP%20Ai%20Controller%20Base) true)
          (Components|Movement|StopMovementImmediately (Variables|Character|GetCharacterMovement))
          (Variables|/Script/Engine.CharacterMovementComponent|SetMaxWalkSpeed (Variables|Character|GetCharacterMovement) (Variables|Default|GetDefault%20Walk%20Speed))
          (Variables|Default|SetTargetPlayer 0)
          (CallFunction|OnAISpawned))))
    (:else
      (goto _label))))

(event Custom|MC_PlayAttackMontage
  (params (MontageToPlay :type Anim%20Montage%20Object%20Reference))
  (Animation|Montage|PlayMontage (Variables|Character|GetMesh) MontageToPlay 0.8
    (:OnBlendOut
      (if (Networking|IsServer)
        (bind _result (Math|Integer|IncrementInt (Variables|Default|GetAnimIndex))
          (:%20%20
            (if (>= _result (Utilities|Array|Length (Variables|Default|GetAllAttackAnim)))
              (Variables|Default|SetAnimIndex 0))
            (CallFunction|AttackLoop)))))))

(event EventTick
  (params (DeltaSeconds :type Float%20%28single-precision%29))
  (CallFunction|DoMeleeTrace))

(event EventPossessed
  (params (NewController :type Controller%20Object%20Reference))
  (bind _asbp_ai_controller_base (Utilities|Casting|CastToBP_Ai_Controller_Base NewController))
  (Variables|Default|SetAs%20BP%20Ai%20Controller%20Base _asbp_ai_controller_base)
  (CallFunction|OnAISpawned)
  (Variables|Default|SetDefault%20Walk%20Speed (Variables|/Script/Engine.CharacterMovementComponent|GetMaxWalkSpeed (Variables|Character|GetCharacterMovement)))
  (CallFunction|MCRemoveClientTrigger))

(fn ConstructionScript)

(fn FindEnemy
  (bind _outactors (Actor|GetAllActorsOfClass "/Game/Characters/BP_Hero_Base.BP_Hero_Base_C"))
  (LocalVariables|SetLcl_AllPlayer _outactors)
  (bind _arrayelement (Utilities|Array|ReverseforEachLoop (LocalVariables|GetLcl_AllPlayer))
    (:LoopBody
      (if (not (Variables|/Game/Characters/BP_Hero_Base.BP_Hero_Base_C|GetIsAlive _arrayelement))
        (Utilities|Array|RemoveItem (LocalVariables|GetLcl_AllPlayer) _arrayelement)))
    (:Completed
      (if (Utilities|Array|IsNotEmpty (LocalVariables|GetLcl_AllPlayer))
        (if (== (Utilities|Array|Length (LocalVariables|GetLcl_AllPlayer)) 1)
          (LocalVariables|SetLcl_IsValidPlayerFound true)
          (LocalVariables|SetLcl_NewEnemy (Utilities|Array|Get(acopy) (LocalVariables|GetLcl_AllPlayer)))
          (else
            (for _array_element (LocalVariables|GetLcl_AllPlayer)
              (Utilities|Array|Add (LocalVariables|GetLcl_AllAttackerNRs) (Variables|/Game/Characters/BP_Hero_Base.BP_Hero_Base_C|GetNRAiAttacker _array_element)))
            (LocalVariables|SetLcl_LowestIndex (.IndexOfMinValue (Math|Integer|MinOfIntArray (LocalVariables|GetLcl_AllAttackerNRs))))
            (if (== (LocalVariables|GetLcl_LowestIndex) -1)
              (LocalVariables|SetLcl_IsValidPlayerFound false)
              (else
                (LocalVariables|SetLcl_NewEnemy (Utilities|Array|Get(acopy) (LocalVariables|GetLcl_AllPlayer) (LocalVariables|GetLcl_LowestIndex)))
                (LocalVariables|SetLcl_IsValidPlayerFound true)))))
        (else
          (LocalVariables|SetLcl_IsValidPlayerFound false)))
      (return (LocalVariables|GetLcl_IsValidPlayerFound) (LocalVariables|GetLcl_NewEnemy)))))

(fn GetDeathMontage
  (params (DamageDirection :type E_DamageDirection%20Enum :default "NewEnumerator0"))
  (switch Utilities|FlowControl|Switch|SwitchonE_DamageDirection DamageDirection
    (:NewEnumerator0
      _)
    (:NewEnumerator1
      _)
    (:NewEnumerator2
      _)
    (:NewEnumerator3
      _))
  (LocalVariables|SetLcl_DeathMonatge "/Game/AnimalVarietyPack/Wolf/Animations/ANIM_Wolf_Death_Montage.ANIM_Wolf_Death_Montage")
  (return (LocalVariables|GetLcl_DeathMonatge)))

(fn SetTargetPlayer
  (params (TargetPlayer :type BP%20Hero%20Base%20Object%20Reference))
  (Utilities|IsValid (Variables|Default|GetTargetPlayer)
    (:Is%20Valid
      (Math|Integer|DecrementInt (Variables|/Game/Characters/BP_Hero_Base.BP_Hero_Base_C|GetNRAiAttacker (Variables|Default|GetTargetPlayer))
        (:%20%20
          _)))
    (:Is%20Not%20Valid
      _))
  (bind _output_get (Variables|Default|SetTargetPlayer TargetPlayer))
  (Math|Integer|IncrementInt (Variables|/Game/Characters/BP_Hero_Base.BP_Hero_Base_C|GetNRAiAttacker _output_get)
    (:%20%20
      (Variables|/Game/AI/Wolf/BP_Ai_Controller_Base.BP_Ai_Controller_Base_C|SetTargetPlayer (Variables|Default|GetAs%20BP%20Ai%20Controller%20Base) (Variables|Default|GetTargetPlayer))
      (return))))

(fn DoMeleeTrace
  (bind _mesh (Variables|Character|GetMesh))
  (if (Variables|Default|GetHeadAttack)
    (bind (_outhit _returnvalue) (Collision|SphereTraceForObjects (Transformation|GetSocketLocation _mesh "Wolf_-HeadSocket") (Transformation|GetSocketLocation _mesh "Wolf_-HeadSocket_0") 15.0 (Utilities|Array|MakeArray "ObjectTypeQuery3") false 0 "ForDuration" true "(R=1.000000,G=0.000000,B=0.000000,A=1.000000)" "(R=0.000000,G=1.000000,B=0.000000,A=1.000000)" 1.0))
    (if _returnvalue
      (if (Utilities|DoesObjectImplementInterface (.HitActor (Collision|BreakHitResult _outhit)) "/Game/Framework/Interface/BPI_Damage_Player.BPI_Damage_Player_C")
        (Variables|Default|SetHeadAttack false)
        (Class|BPIDamagePlayer|PlayerTakeDamage(Message) (.HitActor (Collision|BreakHitResult _outhit)) self _outhit 1e+01)
        (else
          (Variables|Default|SetHeadAttack false))))))

(fn TakeDamage
  (params (Attacker :type Actor%20Object%20Reference) (Amount :type Float%20%28double-precision%29) (HitBoneName :type Name :default "None") (HitLocation :type Vector :default "0, 0, 0"))
  (if (Variables|Default|GetIsAlive)
    (LocalVariables|SetLcl_IsValidHit true)
    (if (== HitBoneName "Wolf_-Head")
      (LocalVariables|SetLcl_IsHeadShot true)
      (else
        (LocalVariables|SetLcl_IsHeadShot false)))
    (bind _output_get (LocalVariables|SetLcl_DamageYaw (Math|Rotator|NormalizeAxis (- (.yaw (Math|Rotator|MakeRotfromZ (- (Transformation|GetActorLocation Attacker) (Transformation|GetActorLocation)))) (- (.yaw (Transformation|GetActorRotation)) (.yaw (Variables|/Script/Engine.SceneComponent|GetRelativeRotation (Variables|Character|GetMesh))))))))
    (if (< _output_get 0.0)
      (if (Math|Float|InRange(Float) (LocalVariables|GetLcl_DamageYaw) -135.0 -45.0 true false)
        (LocalVariables|SetLcl_DamageDirection "NewEnumerator2")
        (elif (>= (LocalVariables|GetLcl_DamageYaw) -45.0)
          (LocalVariables|SetLcl_DamageDirection "NewEnumerator0")
          (else
            (LocalVariables|SetLcl_DamageDirection "NewEnumerator1"))))
      (elif (Math|Float|InRange(Float) (LocalVariables|GetLcl_DamageYaw) 45.0 135.0 false)
        (LocalVariables|SetLcl_DamageDirection "NewEnumerator3")
        (elif (<= (LocalVariables|GetLcl_DamageYaw) 45.0)
          (LocalVariables|SetLcl_DamageDirection "NewEnumerator0")
          (else
            (LocalVariables|SetLcl_DamageDirection "NewEnumerator1")))))
    (if (LocalVariables|GetLcl_IsHeadShot)
      (LocalVariables|SetLcl_Damage (* Amount 2.0))
      (else
        (LocalVariables|SetLcl_Damage Amount)))
    (bind _output_get_2 (Variables|Default|SetHealth (- (Variables|Default|GetHealth) (LocalVariables|GetLcl_Damage))))
    (Development|PrintString (Utilities|String|ToString(Float) (Variables|Default|GetHealth)))
    (if (<= _output_get_2 0.0)
      (Variables|Default|SetIsAlive false)
      (CallFunction|Die (LocalVariables|GetLcl_DamageDirection)))
    (else
      (LocalVariables|SetLcl_IsValidHit false)))
  (return (not (Variables|Default|GetIsAlive)) (Variables|Default|GetXPWhenKilled) (LocalVariables|GetLcl_IsValidHit)))