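; Weapon effects actor that plays muzzle flash, shell eject and tracer Niagara systems when WeaponFired receives impact positions.
; Each system spawns at its weapon socket if missing or inactive; otherwise it is reused, with a flipped User.Trigger bool signaling each shot.
; The first impact aims the flash, while tracers receive the whole array.
; A retriggerable delay loop destroys the actor once all three auto-destroying systems are gone.
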(event Custom|WeaponFired
  (params (ImpactPositions :type Array%20of%20Vectors))
  (bind _weaponmesh (Variables|Default|GetWeaponMesh))
  (bind _muzzlesocket (Variables|Default|GetMuzzleSocket))
  (bind _returnvalue (Transformation|GetSocketTransform _weaponmesh _muzzlesocket "RTS_World"))
  (bind (_location _rotation) (Math|Transform|BreakTransform _returnvalue))
  (Variables|Default|SetImpact%20Positions ImpactPositions)
  (Utilities|FlowControl|Sequence
    (:then_0
      (Utilities|IsValid (Variables|Default|GetNS_MuzzleFlash)
        (:Is%20Valid
          (if (Components|Activation|IsActive (Variables|Default|GetNS_MuzzleFlash))
            _
            (else
              (bind _returnvalue_2 (Niagara|SpawnSystemAttached (Variables|Default|GetMuzzleFlashFX) (Variables|Default|GetDefaultSceneRoot) "None" _location _rotation "KeepWorldPosition" true :!label _label))
              (Variables|Default|SetNS_MuzzleFlash _returnvalue_2)
              (Variables|Default|SetMuzzleFlashTrigger false))))
        (:Is%20Not%20Valid
          (goto _label)))
      (Variables|Default|SetMuzzleFlashTrigger (not (Variables|Default|GetMuzzleFlashTrigger)))
      (Niagara|SetNiagaraVariable(Vector3) (Variables|Default|GetNS_MuzzleFlash) "User.Direction" (Math|Vector|Normalize (- (Utilities|Array|Get(acopy) (Variables|Default|GetImpact%20Positions)) (.Location (Math|Transform|BreakTransform (Transformation|GetSocketTransform (Variables|Default|GetWeaponMesh) (Variables|Default|GetMuzzleSocket) "RTS_World"))))))
      (Class|NiagaraComponent|SetVariableBool (Variables|Default|GetNS_MuzzleFlash) "User.Trigger" (Variables|Default|GetMuzzleFlashTrigger)))
    (:then_1
      (Utilities|IsValid (Variables|Default|GetNS_ShellEject)
        (:Is%20Valid
          (if (Components|Activation|IsActive (Variables|Default|GetNS_ShellEject))
            _
            (else
              (bind _returnvalue_3 (Niagara|SpawnSystemAttached "/Game/Effects/Particles/Weapons/NS_WeaponFire_ShellEject.NS_WeaponFire_ShellEject" (Variables|Default|GetDefaultSceneRoot) "None" (.Location (Math|Transform|BreakTransform (Transformation|GetSocketTransform (Variables|Default|GetWeaponMesh) (Variables|Default|GetShellEjectSocket) "RTS_World"))) "0.000000,0.000000,0.000000" "KeepWorldPosition" true :!label _label_2))
              (bind _output_get (Variables|Default|SetNS_ShellEject _returnvalue_3))
              (Class|NiagaraComponent|SetVariableStaticMesh _output_get "User.ShellEjectStaticMesh" (Variables|Default|GetShellEjectMesh))
              (Variables|Default|SetShellEjectTrigger false))))
        (:Is%20Not%20Valid
          (goto _label_2)))
      (Variables|Default|SetShellEjectTrigger (not (Variables|Default|GetShellEjectTrigger)))
      (Class|NiagaraComponent|SetVariableBool (Variables|Default|GetNS_ShellEject) "User.Trigger" (Variables|Default|GetShellEjectTrigger)))
    (:then_2
      (Utilities|IsValid (Variables|Default|GetNS_TracerFX)
        (:Is%20Valid
          (if (Components|Activation|IsActive (Variables|Default|GetNS_TracerFX))
            _
            (else
              (bind _returnvalue_4 (Niagara|SpawnSystemAttached (Variables|Default|GetTracerFX) (Variables|Default|GetDefaultSceneRoot) "None" (.Location (Math|Transform|BreakTransform (Transformation|GetSocketTransform (Variables|Default|GetWeaponMesh) (Variables|Default|GetMuzzleSocket) "RTS_World"))) "0.000000,0.000000,0.000000" "KeepWorldPosition" true :!label _label_3))
              (Variables|Default|SetNS_TracerFX _returnvalue_4)
              (Variables|Default|SetTracerTrigger false))))
        (:Is%20Not%20Valid
          (goto _label_3)))
      (Variables|Default|SetTracerTrigger (not (Variables|Default|GetTracerTrigger)))
      (Class|NiagaraDataInterfaceArrayFunctionLibrary|SetNiagaraArrayVector (Variables|Default|GetNS_TracerFX) "User.ImpactPositions" (Variables|Default|GetImpact%20Positions))
      (Class|NiagaraComponent|SetVariableBool (Variables|Default|GetNS_TracerFX) "User.Trigger" (Variables|Default|GetTracerTrigger)))
    (:then_3
      (Utilities|FlowControl|RetriggerableDelay 3.0 :!label _label_4)
      (if (Math|Boolean|ORBoolean (Utilities|IsValid (Variables|Default|GetNS_MuzzleFlash)) (Utilities|IsValid (Variables|Default|GetNS_ShellEject)) (Utilities|IsValid (Variables|Default|GetNS_TracerFX)))
        (goto _label_4)
        (else
          (Actor|DestroyActor))))))

(fn ConstructionScript)