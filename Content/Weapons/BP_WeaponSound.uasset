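; Weapon sound actor that plays a weapon's fire audio through one reusable audio component attached to the weapon mesh.
; WeaponFired spawns the sound only when none is active, passing fire time as ShotInterval, then sends a "Fire" trigger parameter on each shot.
; A retriggerable delay restarts with every shot, then polls the component and destroys the actor once it is no longer valid.
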(event Custom|WeaponFired
  (params (WeaponMeshComp :type Skeletal%20Mesh%20Component%20Object%20Reference) (FireTime :type Float%20%28double-precision%29) (FireSound :type Meta%20Sound%20Source%20Object%20Reference))
  (Variables|Default|SetWeapon%20Mesh%20Comp WeaponMeshComp)
  (Variables|Default|SetFire%20Time FireTime)
  (Variables|Default|SetFire%20Sound FireSound)
  (Utilities|FlowControl|Sequence
    (:then_0
      (Utilities|IsValid (Variables|Default|GetAudioWpnFireComp)
        (:Is%20Valid
          (if (Components|Activation|IsActive (Variables|Default|GetAudioWpnFireComp))
            _
            (else
              (bind _returnvalue (Audio|SpawnSoundAttached (Variables|Default|GetFire%20Sound) (Variables|Default|GetWeapon%20Mesh%20Comp) "None" "0, 0, 0" "0, 0, 0" "KeepRelativeOffset" false 0.5 1.0 0.0 0 0 :!label _label))
              (bind _output_get (Variables|Default|SetAudioWpnFireComp _returnvalue))
              (Audio|Parameter|SetFloatParameter _output_get "ShotInterval" (Variables|Default|GetFire%20Time) :!class /Script/AudioExtensions.AudioParameterControllerInterface))))
        (:Is%20Not%20Valid
          (goto _label)))
      (Class|AudioParameterControllerInterface|SetTriggerParameter (Variables|Default|GetAudioWpnFireComp) "Fire"))
    (:then_1
      (Utilities|FlowControl|RetriggerableDelay 3.0 :!label _label_2)
      (if (Utilities|IsValid (Variables|Default|GetAudioWpnFireComp))
        (goto _label_2)
        (else
          (Actor|DestroyActor))))))

(fn ConstructionScript)