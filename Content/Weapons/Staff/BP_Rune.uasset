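; BP_Rune is a temporary staff-spell rune that boosts the hero's damage while the hero stands inside its Box.
; On BeginPlay it spawns a ground decal at its transform and starts two timers: a short one that enables Box overlap events, and one matching the decal's lifespan.
; Box overlaps call BoostDamage and ResetDamage on BPHero.
; When the spell ends, it resets the hero's damage unconditionally and destroys itself.
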(event OnComponentBeginOverlap(Box)
  (params (OverlappedComponent :type Primitive%20Component%20Object%20Reference) (OtherActor :type Actor%20Object%20Reference) (OtherComp :type Primitive%20Component%20Object%20Reference) (OtherBodyIndex :type Integer) (bFromSweep :type Boolean) (SweepResult :type Hit%20Result%20Structure%20%28by%20ref%29))
  (bind _bp_hero (Variables|Default|GetBP_Hero))
  (if (== OtherActor _bp_hero)
    (Default|BoostDamage _bp_hero 2.0)))

(event OnComponentEndOverlap(Box)
  (params (OverlappedComponent :type Primitive%20Component%20Object%20Reference) (OtherActor :type Actor%20Object%20Reference) (OtherComp :type Primitive%20Component%20Object%20Reference) (OtherBodyIndex :type Integer))
  (bind _bp_hero (Variables|Default|GetBP_Hero))
  (if (== OtherActor _bp_hero)
    (Default|ResetDamage _bp_hero 2.0)))

(event Custom|EndSpell
  (Default|ResetDamage (Variables|Default|GetBP_Hero) 2.0)
  (Actor|DestroyActor))

(event Custom|EventOver
  (Variables|/Script/Engine.PrimitiveComponent|SetbGenerateOverlapEvents (Variables|Default|GetBox) true))

(event EventBeginPlay
  (Rendering|Decal|SpawnDecalatLocation "/Engine/EngineMaterials/DefaultDecalMaterial.DefaultDecalMaterial" "100.000000,100.000000,100.000000" (Transformation|GetActorLocation) (Transformation|GetActorRotation) 1e+01)
  (Utilities|Time|SetTimerbyEvent (delegate Custom|EndSpell) 1e+01)
  (Utilities|Time|SetTimerbyEvent (delegate Custom|EventOver) 1.0))

(event EventTick
  (params (DeltaSeconds :type Float%20%28single-precision%29)))

(fn ConstructionScript)