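; Base projectile Blueprint that applies damage through interfaces when its collision sphere hits an actor.
; SvrProcessHit sends damage with bone and location to BPI_Damage_Interface targets, awarding XP on kills, and damages BPI_Damage_Player targets only in PVP mode.
; Other hits start a two-second timer with no event shown bound, and nothing here calls DestroyProjectiles.
; A Velocity event sets movement velocity from VelocityDirection and prints it.
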(event OnComponentHit(SphereCollision)
  (params (HitComponent :type Primitive%20Component%20Object%20Reference) (OtherActor :type Actor%20Object%20Reference) (OtherComp :type Primitive%20Component%20Object%20Reference) (NormalImpulse :type Vector :default "0, 0, 0") (Hit :type Hit%20Result%20Structure%20%28by%20ref%29))
  (if (Utilities|DoesObjectImplementInterface OtherActor "/Game/Framework/Interface/BPI_Damage_Player.BPI_Damage_Player_C")
    (CallFunction|SvrProcessHit Hit :!label _label)
    (elif (Utilities|DoesObjectImplementInterface OtherActor "/Game/Framework/Interface/BPI_Damage_Interface.BPI_Damage_Interface_C")
      (goto _label)
      (else
        (Utilities|Time|SetTimerbyEvent 0 2.0)))))

(event Custom|DestroyProjectiles
  (Actor|DestroyActor))

(event Custom|Velocity
  (bind _output_get (Variables|/Script/Engine.MovementComponent|SetVelocity (Variables|Default|GetProjectileMovement) (Variables|Default|GetVelocityDirection)))
  (Development|PrintString (Utilities|String|ToString(Vector) _output_get)))

(fn ConstructionScript)

(fn SvrProcessHit
  (params (Hit :type Hit%20Result%20Structure))
  (bind (_bblockinghit _binitialoverlap _time _distance _location _impactpoint _normal _impactnormal _physmat _hitactor _hitcomponent _hitbonename) (Collision|BreakHitResult Hit))
  (if (and _bblockinghit (Utilities|DoesObjectImplementInterface _hitactor "/Game/Framework/Interface/BPI_Damage_Interface.BPI_Damage_Interface_C"))
    (bind (_isdead _xp _isvalidhit) (Class|BPIDamageInterface|TakeDamage(Message) _hitactor self (Variables|Default|GetDamage) _hitbonename _location))
    (if _isvalidhit
      (if _isdead
        (Default|AddXP (Variables|Default|GetBP%20XPComponent) _xp))
      (return))
    (elif (and (Utilities|DoesObjectImplementInterface _hitactor "/Game/Framework/Interface/BPI_Damage_Player.BPI_Damage_Player_C") (Variables|Default|GetIsPVPMode))
      (Class|BPIDamagePlayer|PlayerTakeDamage(Message) _hitactor self "" (Variables|Default|GetDamage) true)
      (return))))