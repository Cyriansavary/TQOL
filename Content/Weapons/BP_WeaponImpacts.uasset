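; Weapon impact effects Blueprint that plays Niagara hit effects by surface type each time the weapon fires.
; WeaponFired sorts hits into body, stone and glass arrays, though a hardcoded branch sends every other non-default surface to stone, leaving glass unreachable.
; Stone and glass each reuse an active Niagara system fed by array parameters.
; Body hits spawn individual sparks, plus randomized damage numbers shown only for the locally controlled owner.
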(event Custom|WeaponFired
  (params (ImpactPositions :type Array%20of%20Vectors) (ImpactNormals :type Array%20of%20Vectors) (ImpactSurfaces :type Array%20of%20EPhysicalSurface%20Enums :default "SurfaceType_Default") (MuzzlePosition :type Vector))
  (bind _glassimpacts (Variables|Default|GetGlassImpacts))
  (bind _stoneimpacts (Variables|Default|GetStoneImpacts))
  (bind _bodyimpacts (Variables|Default|GetBodyImpacts))
  (bind _output (Utilities|Array|Get(acopy) _glassimpacts))
  (bind _output_2 (Utilities|Array|Get(acopy) _stoneimpacts))
  (bind _output_3 (Utilities|Array|Get(acopy) _bodyimpacts))
  (Variables|Default|SetImpact%20Positions ImpactPositions)
  (Variables|Default|SetImpact%20Normals ImpactNormals)
  (Variables|Default|SetImpact%20Surfaces ImpactSurfaces)
  (Variables|Default|SetMuzzle%20Position MuzzlePosition)
  (CallFunction|SplitArraybySurface)
  (Utilities|FlowControl|Sequence
    (:then_0
      (if (Utilities|Array|IsNotEmpty (Variables|Default|GetStoneImpacts))
        (Utilities|IsValid (Variables|Default|GetNS_Stone)
          (:Is%20Valid
            (if (Components|Activation|IsActive (Variables|Default|GetNS_Stone))
              (Transformation|SetWorldLocation (Variables|Default|GetNS_Stone) _output_2 false false)
              (else
                (bind _returnvalue (Niagara|SpawnSystematLocation "/Game/Effects/Particles/Impacts/NS_ImpactConcrete.NS_ImpactConcrete" _output_2 :!label _label))
                (Variables|Default|SetNS_Stone _returnvalue))))
          (:Is%20Not%20Valid
            (goto _label)))
        (Class|NiagaraDataInterfaceArrayFunctionLibrary|SetNiagaraArrayPosition (Variables|Default|GetNS_Stone) "User.ImpactPositions" (Variables|Default|GetStoneImpacts))
        (Class|NiagaraDataInterfaceArrayFunctionLibrary|SetNiagaraArrayVector (Variables|Default|GetNS_Stone) "User.ImpactNormals" (Variables|Default|GetStoneNormals))
        (Class|NiagaraComponent|SetVariableInt (Variables|Default|GetNS_Stone) "User.NumberOfHits" (Utilities|Array|Length (Variables|Default|GetStoneImpacts)))
        (Class|NiagaraComponent|SetVariablePosition (Variables|Default|GetNS_Stone) "User.MuzzlePosition" (Variables|Default|GetMuzzle%20Position))
        (Components|Activation|Activate (Variables|Default|GetNS_Stone) false)))
    (:then_1
      (if (Utilities|Array|IsNotEmpty (Variables|Default|GetGlassImpacts))
        (Utilities|IsValid (Variables|Default|GetNS_Glass)
          (:Is%20Valid
            (if (Components|Activation|IsActive (Variables|Default|GetNS_Glass))
              (Transformation|SetWorldLocation (Variables|Default|GetNS_Glass) _output false false)
              (else
                (bind _returnvalue_2 (Niagara|SpawnSystematLocation "/Game/Effects/Particles/Impacts/NS_ImpactGlass.NS_ImpactGlass" _output :!label _label_2))
                (Variables|Default|SetNS_Glass _returnvalue_2))))
          (:Is%20Not%20Valid
            (goto _label_2)))
        (Class|NiagaraDataInterfaceArrayFunctionLibrary|SetNiagaraArrayPosition (Variables|Default|GetNS_Glass) "User.ImpactPositions" (Variables|Default|GetGlassImpacts))
        (Class|NiagaraDataInterfaceArrayFunctionLibrary|SetNiagaraArrayVector (Variables|Default|GetNS_Glass) "User.ImpactNormals" (Variables|Default|GetGlassNormals))
        (Class|NiagaraComponent|SetVariableInt (Variables|Default|GetNS_Glass) "User.NumberOfHits" (Utilities|Array|Length (Variables|Default|GetGlassImpacts)))
        (Class|NiagaraComponent|SetVariablePosition (Variables|Default|GetNS_Glass) "User.MuzzlePosition" (Variables|Default|GetMuzzle%20Position))
        (Components|Activation|Activate (Variables|Default|GetNS_Glass) false)))
    (:then_2
      (if (Utilities|Array|IsNotEmpty (Variables|Default|GetBodyImpacts))
        (for (_array_element _array_index) (Variables|Default|GetBodyImpacts)
          (Utilities|Array|SetArrayElem (Variables|Default|GetDamageInfo) _array_index (Math|Vector4|MakeVector4 (.X (Math|Vector|BreakVector _array_element)) (.Y (Math|Vector|BreakVector _array_element)) (.Y (Math|Vector|BreakVector _array_element)) (Math|Conversions|ToFloat(Integer) (Math|Random|RandomIntegerinRange 8 12))) true)
          (Niagara|SpawnSystematLocation "/Game/Effects/Particles/Impacts/NS_ImactSparksCharacter.NS_ImactSparksCharacter" _array_element (Math|Conversions|RotationFromXVector (Utilities|Array|Get(acopy) (Variables|Default|GetBodyNormals) _array_index))))
        (if (Pawn|IsLocallyControlled (Variables|Default|GetOwningPlayer))
          (Utilities|IsValid (Variables|Default|GetNS_DamageNumber)
            (:Is%20Valid
              (if (Components|Activation|IsActive (Variables|Default|GetNS_DamageNumber))
                (Transformation|SetWorldLocation (Variables|Default|GetNS_DamageNumber) _output_3 false false)
                (else
                  (bind _returnvalue_3 (Niagara|SpawnSystematLocation "/Game/Effects/Particles/Impacts/NS_DamageNumbers.NS_DamageNumbers" _output_3 :!label _label_3))
                  (Variables|Default|SetNS_DamageNumber _returnvalue_3))))
            (:Is%20Not%20Valid
              (goto _label_3)))
          (Class|NiagaraDataInterfaceArrayFunctionLibrary|SetNiagaraArrayVector4 (Variables|Default|GetNS_DamageNumber) "User.DamageInfo" (Variables|Default|GetDamageInfo))
          (Class|NiagaraComponent|SetVariableBool (Variables|Default|GetNS_DamageNumber) "None" false))))))

(fn ConstructionScript)

(fn SplitArraybySurface
  (for (_array_element _array_index) (Variables|Default|GetImpact%20Surfaces)
    (if (not (Utilities|Enum|Equal(Enum) _array_element "SurfaceType_Default"))
      (if (Utilities|Enum|Equal(Enum) _array_element "SurfaceType1")
        (Utilities|Array|Add (Variables|Default|GetBodyImpacts) (Utilities|Array|Get(acopy) (Variables|Default|GetImpact%20Positions) _array_index))
        (Utilities|Array|Add (Variables|Default|GetBodyNormals) (Utilities|Array|Get(acopy) (Variables|Default|GetImpact%20Normals) _array_index))
        (elif true
          (Utilities|Array|Add (Variables|Default|GetStoneImpacts) (Utilities|Array|Get(acopy) (Variables|Default|GetImpact%20Positions)))
          (Utilities|Array|Add (Variables|Default|GetStoneNormals) (Utilities|Array|Get(acopy) (Variables|Default|GetImpact%20Normals) _array_index))
          (elif (Utilities|Enum|Equal(Enum) _array_element "SurfaceType3")
            (Utilities|Array|Add (Variables|Default|GetGlassImpacts) (Utilities|Array|Get(acopy) (Variables|Default|GetImpact%20Positions)))
            (Utilities|Array|Add (Variables|Default|GetGlassNormals) (Utilities|Array|Get(acopy) (Variables|Default|GetImpact%20Normals) _array_index)))))))
  (return))