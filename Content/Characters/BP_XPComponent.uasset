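; Hero XP component that tracks player XP and level, initialized from the shooter PlayerController's player profile.
; Added XP, processed on the server or locally controlled hero, is checked against a level threshold map capped at level 10.
; Results are written back to the controller's profile; the local player also refreshes the HUD, saves, and plays a level-up animation when earned.
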(event Custom|XP_Component_Init
  (CallFunction|SetupXPMap)
  (bind _asbp_hero_base (Utilities|Casting|CastToBP_Hero_Base (Components|GetOwner)))
  (Variables|Default|SetAs%20BP%20Hero%20Base _asbp_hero_base)
  (bind _asbp_shooter_player_controller (Utilities|Casting|CastToBP_Shooter_PlayerController (Game|GetPlayerController 0)))
  (bind _output_get (Variables|Default|SetAs%20BP%20Shooter%20Player%20Controller _asbp_shooter_player_controller))
  (Variables|Default|SetPlayer%20XP (.player_xp (Variables|/Game/Framework/BP_Shooter_PlayerController.BP_Shooter_PlayerController_C|GetS%20Player%20Profile _output_get)))
  (Variables|Default|SetPlayer%20Level (.player_level (Variables|/Game/Framework/BP_Shooter_PlayerController.BP_Shooter_PlayerController_C|GetS%20Player%20Profile _output_get)))
  (if true
    (Default|UpdXPAmount (Variables|/Game/Framework/BP_Shooter_PlayerController.BP_Shooter_PlayerController_C|GetWB_IngameHUD (Variables|Default|GetAs%20BP%20Shooter%20Player%20Controller)))
    (Default|UpdXPLevel (Variables|/Game/Framework/BP_Shooter_PlayerController.BP_Shooter_PlayerController_C|GetWB_IngameHUD (Variables|Default|GetAs%20BP%20Shooter%20Player%20Controller)))
    (Default|SaveXPandLevel (Variables|Default|GetAs%20BP%20Shooter%20Player%20Controller))))

(event Custom|Add_XP
  (params (XPAmount :type Integer))
  (bind _as_bp_hero_base (Variables|Default|GetAs%20BP%20Hero%20Base))
  (bind _as_bp_shooter_player_controller (Variables|Default|GetAs%20BP%20Shooter%20Player%20Controller))
  (bind _wb_ingame_hud (Variables|/Game/Characters/BP_Hero_Base.BP_Hero_Base_C|GetWB%20Ingame%20HUD _as_bp_hero_base))
  (if (or (Networking|IsServer) (Pawn|IsLocallyControlled (Variables|Default|GetAs%20BP%20Hero%20Base)))
    (bind _output_get (Variables|Default|SetPlayer%20XP (+ (Variables|Default|GetPlayer%20XP) XPAmount)))
    (bind (_canlevelup _newlevel) (CallFunction|CheckforLevelUp _output_get))
    (if _canlevelup
      (Variables|Default|SetPlayer%20Level _newlevel))
    (CallFunction|UpdPlayerControllerProfile)
    (if (Pawn|IsLocallyControlled _as_bp_hero_base)
      (Default|UpdXPAmount _wb_ingame_hud)
      (Default|UpdXPLevel _wb_ingame_hud)
      (Default|SaveXPandLevel _as_bp_shooter_player_controller)
      (if _canlevelup
        (Default|PlayUIAnimLevelUp (Variables|/Game/Framework/BP_Shooter_PlayerController.BP_Shooter_PlayerController_C|GetWB_IngameHUD _as_bp_shooter_player_controller))))))

(fn SetupXPMap
  (Variables|Default|SetXP_Map_Level (.xp_map_levels (LocalVariables|GetS_XPandLevel)))
  (return))

(fn CheckforLevelUp
  (params (XPAmount :type Integer))
  (LocalVariables|SetLcl_CurrentXP XPAmount)
  (LocalVariables|SetLcl_CurrentLevel (Variables|Default|GetPlayer%20Level))
  (if (and (> (LocalVariables|GetLcl_CurrentXP) (Utilities|Array|Get(acopy) (Variables|Default|GetXP_Map_Level) (LocalVariables|GetLcl_CurrentLevel))) (< (LocalVariables|GetLcl_CurrentLevel) 10))
    (LocalVariables|SetLcl_CanLevelUp true)
    (bind _index (Utilities|FlowControl|ForLoopwithBreak (LocalVariables|GetLcl_CurrentLevel) 10 :!label _label)
      (:LoopBody
        (if (not (> (LocalVariables|GetLcl_CurrentXP) (Utilities|Array|Get(acopy) (Variables|Default|GetXP_Map_Level) _index)))
          (LocalVariables|SetLcl_CurrentLevel _index)
          (goto _label Break)))
      (:Completed
        (return (LocalVariables|GetLcl_CanLevelUp) (LocalVariables|GetLcl_CurrentLevel))))
    (else
      (LocalVariables|SetLcl_CanLevelUp false)
      (return (LocalVariables|GetLcl_CanLevelUp) (LocalVariables|GetLcl_CurrentLevel)))))

(fn UpdPlayerControllerProfile
  (bind _as_bp_shooter_player_controller (Variables|Default|GetAs%20BP%20Shooter%20Player%20Controller))
  (Variables|/Game/Framework/BP_Shooter_PlayerController.BP_Shooter_PlayerController_C|SetS%20Player%20Profile _as_bp_shooter_player_controller (Utilities|Struct|MakeS_PlayerProfil (.playername (Variables|/Game/Framework/BP_Shooter_PlayerController.BP_Shooter_PlayerController_C|GetS%20Player%20Profile _as_bp_shooter_player_controller)) (.charrowname (Variables|/Game/Framework/BP_Shooter_PlayerController.BP_Shooter_PlayerController_C|GetS%20Player%20Profile _as_bp_shooter_player_controller)) (.characterclass (Variables|/Game/Framework/BP_Shooter_PlayerController.BP_Shooter_PlayerController_C|GetS%20Player%20Profile _as_bp_shooter_player_controller)) (.modelname (Variables|/Game/Framework/BP_Shooter_PlayerController.BP_Shooter_PlayerController_C|GetS%20Player%20Profile _as_bp_shooter_player_controller)) (.skinname (Variables|/Game/Framework/BP_Shooter_PlayerController.BP_Shooter_PlayerController_C|GetS%20Player%20Profile _as_bp_shooter_player_controller)) (Variables|Default|GetPlayer%20XP) (Variables|Default|GetPlayer%20Level) (.wpn_loadout (Variables|/Game/Framework/BP_Shooter_PlayerController.BP_Shooter_PlayerController_C|GetS%20Player%20Profile _as_bp_shooter_player_controller)) (.wpn_inventory (Variables|/Game/Framework/BP_Shooter_PlayerController.BP_Shooter_PlayerController_C|GetS%20Player%20Profile _as_bp_shooter_player_controller))))
  (return))