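; Lobby game mode for the shooter's menu that tracks connected menu controllers, ready states and profiles, plus the selected gamemode.
; UpdateLobby copies profiles into player states and pushes flagged changes (names, level, characters, ready, gamemode) to every controller.
; Each player gets a lobby character spawned on a free spot, dressed from a customization DataTable via MC calls, while previews use Client calls.
; Logout destroys the character and frees its spot.
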(event Custom|UpdateLobby
  (params (PlayerName :type Boolean) (LevelSelection :type Boolean) (CharacterSelection :type Boolean) (PlayerReady :type Boolean) (Gamemode :type Boolean))
  (Utilities|Array|Clear (Variables|Default|GetAll_PlayerProfile))
  (for (_array_element _array_index) (Variables|Default|GetALL_ConnectedPlayer)
    (Utilities|Array|SetArrayElem (Variables|Default|GetAll_PlayerProfile) _array_index (Variables|/Game/Framework/BP_Menu_Controller.BP_Menu_Controller_C|GetPLayer%20Profile%20Info _array_element) true)
    (bind _asbp_shooter_player_state (Utilities|Casting|CastToBP_Shooter_PlayerState (Variables|/Script/Engine.Controller|GetPlayerState _array_element)))
    (Variables|/Game/Framework/BP_Shooter_PlayerState.BP_Shooter_PlayerState_C|SetS_PlayerProfile _asbp_shooter_player_state (Variables|/Game/Framework/BP_Menu_Controller.BP_Menu_Controller_C|GetPLayer%20Profile%20Info _array_element)))
  (for (_array_element_2 _array_index_2) (Variables|Default|GetALL_ConnectedPlayer)
    (if PlayerName
      (Default|UpdatePlayerNames _array_element_2 (Variables|Default|GetAll_PlayerProfile)))
    (if LevelSelection
      (Default|UpdateLevelSelection _array_element_2 (Variables|Default|GetLevelSelectedName)))
    (if CharacterSelection
      (CallFunction|UpdateSelectedCharacter _array_index_2))
    (if PlayerReady
      (Default|UpdatePlayerReady _array_element_2 (Variables|Default|GetIsPlayerReady)))
    (if Gamemode
      (Default|UpdateGamemode _array_element_2 (Variables|Default|GetSelectedGameode)))))

(event Custom|UpdateSelectedCharacter
  (params (PlayerIndex :type Integer))
  (bind _all_connectedplayer (Variables|Default|GetALL_ConnectedPlayer))
  (bind _all_connectedplayer_2 (Variables|Default|GetALL_ConnectedPlayer))
  (bind _all_playerprofile (Variables|Default|GetAll_PlayerProfile))
  (bind _output (Utilities|Array|Get(acopy) _all_connectedplayer PlayerIndex))
  (bind _output_2 (Utilities|Array|Get(acopy) _all_connectedplayer_2 PlayerIndex))
  (bind _output_3 (Utilities|Array|Get(acopy) _all_playerprofile PlayerIndex))
  (if (== (Variables|/Game/Framework/BP_Menu_Controller.BP_Menu_Controller_C|GetLobbyCharacter_BP _output) 0)
    (bind _availableplayerspot (CallFunction|GetPlayerLobbySpot))
    (Variables|/Game/Gameplay/Lobby/BP_Lobby_PlayerSpot.BP_Lobby_PlayerSpot_C|SetIsSpotUsed _availableplayerspot true)
    (bind _returnvalue (Game|SpawnActorfromClass "/Game/Gameplay/Lobby/BP_Lobby_Character.BP_Lobby_Character_C" (Transformation|GetActorTransform _availableplayerspot) "Undefined" "MultiplyWithRoot" _output 0))
    (Variables|/Game/Framework/BP_Menu_Controller.BP_Menu_Controller_C|SetLobbyCharacter_BP _output_2 _returnvalue)
    (Variables|/Game/Framework/BP_Menu_Controller.BP_Menu_Controller_C|SetLobbyPlayerSpot_BP _output_2 _availableplayerspot))
  (Default|MCSetPlayerName (Variables|/Game/Framework/BP_Menu_Controller.BP_Menu_Controller_C|GetLobbyCharacter_BP (Utilities|Array|Get(acopy) (Variables|Default|GetALL_ConnectedPlayer) PlayerIndex)) (.playername _output_3))
  (bind _returnvalue_2 (Utilities|GetDataTableRow "/Game/Characters/CharacterCustumisation_Table.CharacterCustumisation_Table" (.charrowname _output_3))
    (:then
      (Default|MCSetCharMesh (Variables|/Game/Framework/BP_Menu_Controller.BP_Menu_Controller_C|GetLobbyCharacter_BP (Utilities|Array|Get(acopy) (Variables|Default|GetALL_ConnectedPlayer) PlayerIndex)) (.Model (Utilities|Struct|BreakS_ModelAndSkin (.Value (Utilities|Map|Find (.MeshAndSkin (Utilities|Struct|BreakS_CharacterCustumisation _returnvalue_2)) (.modelname _output_3))))))
      (Default|MCPlayeMeshAnim (Variables|/Game/Framework/BP_Menu_Controller.BP_Menu_Controller_C|GetLobbyCharacter_BP (Utilities|Array|Get(acopy) (Variables|Default|GetALL_ConnectedPlayer) PlayerIndex)) (.LobbyAnimation (Utilities|Struct|BreakS_ModelAndSkin (.Value (Utilities|Map|Find (.MeshAndSkin (Utilities|Struct|BreakS_CharacterCustumisation _returnvalue_2)) (.modelname _output_3))))))
      (if (.Use_Skin0 (Utilities|Struct|BreakS_ModelAndSkin (.Value (Utilities|Map|Find (.MeshAndSkin (Utilities|Struct|BreakS_CharacterCustumisation _returnvalue_2)) (.modelname _output_3)))))
        (Default|MCSetSkinMaterial (Variables|/Game/Framework/BP_Menu_Controller.BP_Menu_Controller_C|GetLobbyCharacter_BP (Utilities|Array|Get(acopy) (Variables|Default|GetALL_ConnectedPlayer) PlayerIndex)) (.Skin0_MaterialSlot (Utilities|Struct|BreakS_ModelAndSkin (.Value (Utilities|Map|Find (.MeshAndSkin (Utilities|Struct|BreakS_CharacterCustumisation _returnvalue_2)) (.modelname _output_3))))) (.Value (Utilities|Map|Find (.Skin0_Skins (Utilities|Struct|BreakS_ModelAndSkin (.Value (Utilities|Map|Find (.MeshAndSkin (Utilities|Struct|BreakS_CharacterCustumisation _returnvalue_2)) (.modelname _output_3))))) (.skinname _output_3)))))
      (if (.Use_Skin1 (Utilities|Struct|BreakS_ModelAndSkin (.Value (Utilities|Map|Find (.MeshAndSkin (Utilities|Struct|BreakS_CharacterCustumisation _returnvalue_2)) (.modelname _output_3)))))
        (Default|MCSetSkinMaterial (Variables|/Game/Framework/BP_Menu_Controller.BP_Menu_Controller_C|GetLobbyCharacter_BP (Utilities|Array|Get(acopy) (Variables|Default|GetALL_ConnectedPlayer) PlayerIndex)) (.Skin1_MaterialSlot (Utilities|Struct|BreakS_ModelAndSkin (.Value (Utilities|Map|Find (.MeshAndSkin (Utilities|Struct|BreakS_CharacterCustumisation _returnvalue_2)) (.modelname _output_3))))) (.Value (Utilities|Map|Find (.Skin1_Skins (Utilities|Struct|BreakS_ModelAndSkin (.Value (Utilities|Map|Find (.MeshAndSkin (Utilities|Struct|BreakS_CharacterCustumisation _returnvalue_2)) (.modelname _output_3))))) (.skinname _output_3))))))))

(event Custom|UpdateCharForController
  (params (Controller :type BP%20Menu%20Controller%20Object%20Reference) (PlayerProfil :type S%20Player%20Profil%20Structure))
  (bind _all_connectedplayer (Variables|Default|GetALL_ConnectedPlayer))
  (bind _returnvalue (Utilities|Array|FindItem _all_connectedplayer Controller))
  (Utilities|Array|SetArrayElem (Variables|Default|GetAll_PlayerProfile) _returnvalue PlayerProfil true)
  (bind _asbp_shooter_player_state (Utilities|Casting|CastToBP_Shooter_PlayerState (Variables|/Script/Engine.Controller|GetPlayerState Controller)))
  (Variables|/Game/Framework/BP_Shooter_PlayerState.BP_Shooter_PlayerState_C|SetS_PlayerProfile _asbp_shooter_player_state PlayerProfil)
  (CallFunction|UpdateSelectedCharacter _returnvalue))

(event Custom|PreviewCharacterForController
  (params (Controller :type BP%20Menu%20Controller%20Object%20Reference) (CharRowName :type Name) (ModelName :type Name) (SkinName :type Name))
  (bind _lobbycharacter_bp (Variables|/Game/Framework/BP_Menu_Controller.BP_Menu_Controller_C|GetLobbyCharacter_BP Controller))
  (bind _returnvalue (Utilities|GetDataTableRow "/Game/Characters/CharacterCustumisation_Table.CharacterCustumisation_Table" CharRowName)
    (:then
      (Default|ClientSetCharacterMesh _lobbycharacter_bp (.Model (Utilities|Struct|BreakS_ModelAndSkin (.Value (Utilities|Map|Find (.MeshAndSkin (Utilities|Struct|BreakS_CharacterCustumisation _returnvalue)) ModelName)))))
      (Default|ClientPlayMeshAnim _lobbycharacter_bp (.LobbyAnimation (Utilities|Struct|BreakS_ModelAndSkin (.Value (Utilities|Map|Find (.MeshAndSkin (Utilities|Struct|BreakS_CharacterCustumisation _returnvalue)) ModelName)))))
      (if (.Use_Skin0 (Utilities|Struct|BreakS_ModelAndSkin (.Value (Utilities|Map|Find (.MeshAndSkin (Utilities|Struct|BreakS_CharacterCustumisation _returnvalue)) ModelName))))
        (Default|ClientSetSkinMaterial _lobbycharacter_bp (.Skin0_MaterialSlot (Utilities|Struct|BreakS_ModelAndSkin (.Value (Utilities|Map|Find (.MeshAndSkin (Utilities|Struct|BreakS_CharacterCustumisation _returnvalue)) ModelName)))) (.Value (Utilities|Map|Find (.Skin0_Skins (Utilities|Struct|BreakS_ModelAndSkin (.Value (Utilities|Map|Find (.MeshAndSkin (Utilities|Struct|BreakS_CharacterCustumisation _returnvalue)) ModelName)))) SkinName))))
      (if (.Use_Skin1 (Utilities|Struct|BreakS_ModelAndSkin (.Value (Utilities|Map|Find (.MeshAndSkin (Utilities|Struct|BreakS_CharacterCustumisation _returnvalue)) ModelName))))
        (Default|ClientSetSkinMaterial _lobbycharacter_bp (.Skin1_MaterialSlot (Utilities|Struct|BreakS_ModelAndSkin (.Value (Utilities|Map|Find (.MeshAndSkin (Utilities|Struct|BreakS_CharacterCustumisation _returnvalue)) ModelName)))) (.Value (Utilities|Map|Find (.Skin1_Skins (Utilities|Struct|BreakS_ModelAndSkin (.Value (Utilities|Map|Find (.MeshAndSkin (Utilities|Struct|BreakS_CharacterCustumisation _returnvalue)) ModelName)))) SkinName)))))))

(event Custom|SetPlayerReady
  (params (PlayerController :type BP%20Menu%20Controller%20Object%20Reference) (IsReady :type Boolean))
  (Utilities|Array|SetArrayElem (Variables|Default|GetIsPlayerReady) (Utilities|Array|FindItem (Variables|Default|GetALL_ConnectedPlayer) PlayerController) IsReady)
  (CallFunction|UpdateLobby false false false true false))

(event Custom|SetSelectedGamemode
  (params (SelectedGameode :type E_GameMode%20Enum :default "NewEnumerator0"))
  (Variables|Default|SetSelectedGameode SelectedGameode)
  (CallFunction|UpdateLobby false false false false true))

(event EventOnLogout
  (params (ExitingController :type Controller%20Object%20Reference))
  (bind _asbp_menu_controller (Utilities|Casting|CastToBP_Menu_Controller ExitingController))
  (if (== (Variables|/Game/Framework/BP_Menu_Controller.BP_Menu_Controller_C|GetLobbyCharacter_BP _asbp_menu_controller) 0)
    _
    (else
      (Actor|DestroyActor (Variables|/Game/Framework/BP_Menu_Controller.BP_Menu_Controller_C|GetLobbyCharacter_BP _asbp_menu_controller))
      (Variables|/Game/Gameplay/Lobby/BP_Lobby_PlayerSpot.BP_Lobby_PlayerSpot_C|SetIsSpotUsed (Variables|/Game/Framework/BP_Menu_Controller.BP_Menu_Controller_C|GetLobbyPlayerSpot_BP _asbp_menu_controller) false)))
  (Utilities|Array|RemoveIndex (Variables|Default|GetIsPlayerReady) (Utilities|Array|FindItem (Variables|Default|GetALL_ConnectedPlayer) _asbp_menu_controller))
  (Utilities|Array|RemoveIndex (Variables|Default|GetALL_ConnectedPlayer) (Utilities|Array|FindItem (Variables|Default|GetALL_ConnectedPlayer) _asbp_menu_controller))
  (CallFunction|UpdateLobby true false true true false))

(event EventHandleStartingNewPlayer
  (params (NewPlayer :type Player%20Controller%20Object%20Reference))
  (bind _returnvalue (Game|GetCurrentLevelName true))
  (switch string _returnvalue
    (:Lobby_Map
      (bind _asbp_menu_controller (Utilities|Casting|CastToBP_Menu_Controller NewPlayer))
      (bind _returnvalue_2 (Utilities|Array|Add (Variables|Default|GetALL_ConnectedPlayer) _asbp_menu_controller))
      (Utilities|Array|SetArrayElem (Variables|Default|GetIsPlayerReady) _returnvalue_2 false true)
      (Default|CreateLobbyMenu _asbp_menu_controller)
      (Default|InitialSetup _asbp_menu_controller))))

(fn ConstructionScript)

(fn GetPlayerLobbySpot
  (if (== (Utilities|Array|Length (Variables|Default|GetALL_Lobby_PlayerSpot)) 0)
    (bind _outactors (Actor|GetAllActorsOfClass "/Game/Gameplay/Lobby/BP_Lobby_PlayerSpot.BP_Lobby_PlayerSpot_C"))
    (Variables|Default|SetALL_Lobby_PlayerSpot _outactors))
  (bind _array_element (Utilities|Array|ForEachLoopwithBreak (Variables|Default|GetALL_Lobby_PlayerSpot) :!label _label)
    (:LoopBody
      (if (not (Variables|/Game/Gameplay/Lobby/BP_Lobby_PlayerSpot.BP_Lobby_PlayerSpot_C|GetIsSpotUsed _array_element))
        (goto _label Break)))
    (:Completed
      (return _array_element))))