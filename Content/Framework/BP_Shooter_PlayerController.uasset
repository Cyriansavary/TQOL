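; Player controller for the multiplayer shooter, handling profile loading and saving, HUD and menus, respawn and post-death spectating.
; The locally loaded save-game profile syncs to the server, and a polling loop marks the player ready once profile, GameState and PlayerState exist.
; Game mode sets respawn, spectate and PvP flags for Free for All or Endless Wave.
; Spectating unpossesses, then cycles view targets through living player heroes.
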(event Custom|EndClientSession
  (bind _self self)
  (bind _asbp_shooter_game_instance (Utilities|Casting|CastToBP_Shooter_GameInstance (Game|GetGameInstance)))
  (Variables|/Game/Framework/BP_Shooter_GameInstance.BP_Shooter_GameInstance_C|SetMp_IsPausedMenuPaused _asbp_shooter_game_instance false)
  (|DestroySession _self
    (:then
      (bind _asbp_shooter_gamemode (Utilities|Casting|CastToBP_Shooter_Gamemode (Game|GetGameMode)))
      (Default|GMPVPGameOver _asbp_shooter_gamemode _self)
      (bind _output_get (Variables|Default|SetS%20Player%20Profile (Utilities|Struct|MakeS_PlayerProfil (.playername (Variables|Default|GetS%20Player%20Profile)) (.charrowname (Variables|Default|GetS%20Player%20Profile)) (.characterclass (Variables|Default|GetS%20Player%20Profile)) (.modelname (Variables|Default|GetS%20Player%20Profile)) (.skinname (Variables|Default|GetS%20Player%20Profile)) (.player_xp (Variables|Default|GetS%20Player%20Profile)) (.player_level (Variables|Default|GetS%20Player%20Profile)) (.wpn_loadout (Variables|Default|GetS%20Player%20Profile)) (.wpn_inventory (Variables|Default|GetS%20Player%20Profile)) (.sensitivity (Variables|Default|GetS%20Player%20Profile)) (+ (.gold (Variables|Default|GetS%20Player%20Profile)) (Variables|/Game/Characters/BP_Hero_Base.BP_Hero_Base_C|GetTempGold (Variables|Default|GetAs%20BP%20Hero%20Base))))))
      (bind _asbp_shooter_game_instance_2 (Utilities|Casting|CastToBP_Shooter_GameInstance (Game|GetGameInstance)))
      (Variables|/Game/Framework/BP_Shooter_GameInstance.BP_Shooter_GameInstance_C|SetPLayer%20Profile _asbp_shooter_game_instance_2 _output_get)
      (Default|SaveProfile _asbp_shooter_game_instance_2))))

(event Custom|GameStartCount
  (Default|GameStartCountdown (Variables|Default|GetWB_IngameHUD)))

(event Custom|ShowSpectatorControls
  (Default|ShowSpectatorControls (Variables|Default|GetWB_PlayerDiedMenu) true)
  (Variables|Default|SetbShowMouseCursor false)
  (Input|SetInputModeGameOnly self false))

(event Custom|UpdateHUD_SpectatorPlayerName
  (params (PlayerName :type Text))
  (Default|UpdateSpectatorName (Variables|Default|GetWB_PlayerDiedMenu) PlayerName))

(event Custom|Svr_GetSpectatorPlayerName
  (params (SpectatorTarget :type BP%20Hero%20Base%20Object%20Reference))
  (CallFunction|UpdateHUDSpectatorPlayerName (.PlayerName (Utilities|Struct|BreakS_PlayerProfil (Variables|BP_Shooter_PlayerController_C|GetS%20Player%20Profile (Variables|/Game/Characters/BP_Hero_Base.BP_Hero_Base_C|GetBP_ShooterPlayerController SpectatorTarget))))))

(event Custom|Svr_Unpossess
  (Pawn|UnPossess))

(event Custom|Svr_ResetTrigger
  (Variables|Default|SetTargetUnPossessed false))

(event Custom|Client_Save_PickedUpWeapon
  (params (WeaponRowName :type Name))
  (CallFunction|SavePickedUpWeapon WeaponRowName))

(event Custom|LoadProfile
  (bind _asbp_shooter_game_instance (Utilities|Casting|CastToBP_Shooter_GameInstance (Game|GetGameInstance)))
  (Variables|Default|SetSlot%20Name (Variables|/Game/Framework/BP_Shooter_GameInstance.BP_Shooter_GameInstance_C|GetSlot%20Name _asbp_shooter_game_instance))
  (bind _returnvalue (SaveGame|LoadGamefromSlot (Variables|Default|GetSlot%20Name)))
  (bind _assg_player_profil (Utilities|Casting|CastToSG_PlayerProfil _returnvalue))
  (Variables|Default|SetAs%20SG%20Player%20Profil _assg_player_profil)
  (Networking|SwitchHasAuthority
    (:Authority
      (Variables|Default|SetS%20Player%20Profile (Variables|/Game/SavedData/SG_PlayerProfil.SG_PlayerProfil_C|GetPlayerProfile _assg_player_profil))
      (Variables|Default|SetIsProfileLoaded true))
    (:Remote
      (CallFunction|SvrSetPlayerProfil (Variables|/Game/SavedData/SG_PlayerProfil.SG_PlayerProfil_C|GetPlayerProfile _assg_player_profil)))))

(event Custom|Svr_CharBeginToPlay
  (bind _asbp_hero_base (Utilities|Casting|CastToBP_Hero_Base (Pawn|GetControlledPawn)))
  (Default|MCBegintoPlay _asbp_hero_base)
  (Variables|Default|SetAs%20BP%20Hero%20Base _asbp_hero_base))

(event Custom|Client_HUD_StartNewWave
  (params (WaveNumber :type Integer))
  (Default|GWEWStartNewWave (Variables|Default|GetWB_IngameHUD) WaveNumber))

(event Custom|Svr_IsRespawningEnable
  (bind _asbp_shooter_gamemode (Utilities|Casting|CastToBP_Shooter_Gamemode (Game|GetGameMode)))
  (switch Utilities|FlowControl|Switch|SwitchonE_GameMode (Variables|/Game/Framework/BP_Shooter_Gamemode.BP_Shooter_Gamemode_C|GetGameMode _asbp_shooter_gamemode)
    (:NewEnumerator1
      (Variables|Default|SetIsRespawningEnable false)
      (Variables|Default|SetIsSpectatingEnabled true)
      (Variables|Default|SetIsPVPMode true))
    (:NewEnumerator2
      (Variables|Default|SetIsRespawningEnable false)
      (Variables|Default|SetIsSpectatingEnabled true)
      (Variables|Default|SetIsPVPMode false))))

(event Custom|UnHide_InGameHUD
  (Widget|SetVisibility (Variables|Default|GetWB_IngameHUD) "Visible"))

(event Custom|ShowGameOverScreen
  (params (WaveSurvived :type Integer) (IsPvPGame :type Boolean) (IsWinner :type Boolean) (IsTimeLimit :type Boolean))
  (Viewport|RemoveAllWidgets)
  (bind _returnvalue (Game|ConstructObjectfromClass self "/Game/Widget/WB_GameOverMenu.WB_GameOverMenu_C" WaveSurvived IsPvPGame IsWinner IsTimeLimit))
  (UserInterface|Viewport|AddtoViewport _returnvalue 0))

(event Custom|OnControllerSpawned
  (if (Variables|Default|GetIsGameStateReady) :!label _label
    _
    (else
      (bind _asbp_game_state (Utilities|Casting|CastToBP_GameState (Game|GetGameState))
        (:then
          (Variables|Default|SetBP_GameState _asbp_game_state)
          (Variables|Default|SetIsGameStateReady true))
        (:CastFailed
          _))))
  (if (Variables|Default|GetIsPlayerStateReady)
    _
    (else
      (bind _asbp_shooter_player_state (Utilities|Casting|CastToBP_Shooter_PlayerState (Variables|GetPlayerState))
        (:then
          (Variables|Default|SetBP_PlayerState _asbp_shooter_player_state)
          (Variables|Default|SetIsPlayerStateReady true))
        (:CastFailed
          _))))
  (if (Math|Boolean|ANDBoolean (Variables|Default|GetIsProfileLoaded) (Variables|Default|GetIsGameStateReady) (Variables|Default|GetIsPlayerStateReady))
    (Variables|Default|SetIsPlayerReady true)
    (else
      (Utilities|FlowControl|Delay 0.1)
      (goto _label))))

(event Custom|HUD_StartMatch_PVP
  (Default|GMPVPStartMatch (Variables|Default|GetWB_IngameHUD)))

(event Custom|HUD_SetupMatchTimer
  (params (TimeLeftSec :type Integer))
  (bind _wb_ingamehud (Variables|Default|GetWB_IngameHUD))
  (Widget|SetVisibility (Variables|/Game/Widget/WB_InGameHUD.WB_InGameHUD_C|GetText_MatchDuration _wb_ingamehud) "Visible")
  (Default|UpdateMatchTimer _wb_ingamehud TimeLeftSec))

(event Custom|SetSpawnRotation
  (params (New%20Rotation%20Z%20%28Yaw%29 :type Float%20%28single-precision%29))
  (Pawn|SetControlRotation (Math|Rotator|MakeRotator 0.0 0.0 New%20Rotation%20Z%20%28Yaw%29)))

(event Custom|Controller_DisableInput
  (Input|DisableInput (Pawn|GetControlledPawn) self))

(event Custom|Client_ToggleScoreboard
  (params (NewVisibility :type Boolean))
  (CallFunction|UIToggleScoreboard NewVisibility))

(event Custom|EnableAllInput
  (Input|EnableInput (Pawn|GetControlledPawn) self))

(event Custom|HUD_SetInteractHint
  (params (NewVisibility :type Boolean) (HintText :type Text))
  (Default|SetInteractableHint (Variables|Default|GetWB_IngameHUD) NewVisibility HintText))

(event Custom|Svr_SetPlayerProfil
  (params (S%20Player%20Profile :type S%20Player%20Profil%20Structure))
  (Variables|Default|SetS%20Player%20Profile S%20Player%20Profile)
  (Variables|Default|SetIsProfileLoaded true))

(event Custom|Save_XPandLevel
  (bind _as_sg_player_profil (Variables|Default|GetAs%20SG%20Player%20Profil))
  (Utilities|FlowControl|RetriggerableDelay 0.5)
  (Variables|/Game/SavedData/SG_PlayerProfil.SG_PlayerProfil_C|SetPlayerProfile _as_sg_player_profil (Variables|Default|GetS%20Player%20Profile))
  (SaveGame|SaveGametoSlot _as_sg_player_profil (Variables|Default|GetSlot%20Name)))

(event Custom|RespawnAfterDeath
  (bind _asbp_shooter_gamemode (Utilities|Casting|CastToBP_Shooter_Gamemode (Game|GetGameMode)))
  (Default|RespawnAfterDying _asbp_shooter_gamemode self))

(event Custom|MC_BeginToPlay
  (if (Pawn|IsLocalPlayerController)
    (Input|SetInputModeGameOnly self false)
    (if (Variables|Default|GetDebugWindow)
      (Variables|Default|SetbShowMouseCursor true :!label _label)
      (Class|PlayerController|ActivateTouchInterface "/Engine/MobileResources/HUD/DefaultVirtualJoysticks.DefaultVirtualJoysticks")
      (else
        (switch string (Game|GetPlatformName)
          (:Default
            (goto _label))
          (:Windows
            (Variables|Default|SetbShowMouseCursor false)
            (Viewport|RemoveAllWidgets))
          (:Android
            (goto _label)))))
    (CallFunction|UIShowinGameHUD)
    (CallFunction|SvrIsRespawningEnable)
    (Networking|SwitchHasAuthority
      (:Authority
        (bind _asbp_hero_base (Utilities|Casting|CastToBP_Hero_Base (Pawn|GetControlledPawn)))
        (Default|MCBegintoPlay _asbp_hero_base)
        (Variables|Default|SetAs%20BP%20Hero%20Base _asbp_hero_base))
      (:Remote
        (CallFunction|SvrCharBegintoPlay)))
    (else
      (Actor|Tick|SetActorTickEnabled false))))

(event Custom|SpectateAfterDeath
  (bind _currentspectatortarget (Variables|Default|GetCurrentSpectatorTarget))
  (Variables|Default|SetIsSpectating true)
  (Networking|SwitchHasAuthority
    (:Authority
      (Pawn|UnPossess))
    (:Remote
      (CallFunction|SvrUnpossess)))
  (if (Variables|Default|GetTargetUnPossessed) :!label _label
    (CallFunction|ShowSpectatorControls)
    (CallFunction|SpectatorUpdateTarget)
    (CallFunction|SpectatorStartSpectateTarget false)
    (Utilities|IsValid _currentspectatortarget
      (:Is%20Valid
        (CallFunction|SvrGetSpectatorPlayerName _currentspectatortarget))
      (:Is%20Not%20Valid
        _))
    (Networking|SwitchHasAuthority
      (:Authority
        (Variables|Default|SetTargetUnPossessed false))
      (:Remote
        (CallFunction|SvrResetTrigger)))
    (else
      (Utilities|FlowControl|DelayUntilNextTick)
      (goto _label))))

(event EventPossess
  (params (PossessedPawn :type Pawn%20Object%20Reference))
  (CallFunction|MCBegintoPlay))

(event EventUnPossess
  (params (UnpossessedPawn :type Pawn%20Object%20Reference))
  (Utilities|FlowControl|Delay 0.1)
  (Variables|Default|SetTargetUnPossessed true))

(event Input|ActionEvents|InputActionPauseGame
  (params (Key :type Key%20Structure))
  (bind _wb_ingamehud (Variables|Default|GetWB_IngameHUD))
  (:Pressed
    (bind _asbp_shooter_game_instance (Utilities|Casting|CastToBP_Shooter_GameInstance (Game|GetGameInstance)))
    (bind _isgamepausedresult (Default|TogglePauseGame _asbp_shooter_game_instance))
    (if _isgamepausedresult
      (if (and (Utilities|IsValid _wb_ingamehud) (UserInterface|Viewport|IsinViewport _wb_ingamehud))
        (Widget|SetVisibility (Variables|Default|GetWB_IngameHUD) "Hidden")))))

(event Input|KeyboardEvents|R
  (params (Key :type Key%20Structure)))

(event Input|KeyboardEvents|A
  (params (Key :type Key%20Structure)))

(event Input|KeyboardEvents|E
  (params (Key :type Key%20Structure)))

(fn ConstructionScript)

(fn UIShowinGameHUD
  (Utilities|IsValid (Variables|Default|GetWB_IngameHUD)
    (:Is%20Valid
      _)
    (:Is%20Not%20Valid
      (bind _returnvalue (UserInterface|CreateWidget "/Game/Widget/WB_InGameHUD.WB_InGameHUD_C" self))
      (Variables|Default|SetWB_IngameHUD _returnvalue)))
  (UserInterface|Viewport|AddtoViewport (Variables|Default|GetWB_IngameHUD) 0)
  (return))

(fn UIShowPlayerDiedMenu
  (bind _wb_ingamehud (Variables|Default|GetWB_IngameHUD))
  (bind _wb_ingamehud_2 (Variables|Default|GetWB_IngameHUD))
  (if (not (Variables|Default|GetIsGameOver))
    (bind _outactors (Actor|GetAllActorsOfClass "/Game/Characters/BP_Hero_Base.BP_Hero_Base_C"))
    (for _array_element _outactors
      (if (not (Variables|/Game/Characters/BP_Hero_Base.BP_Hero_Base_C|GetIsAlive _array_element))
        (Math|Integer|IncrementInt (LocalVariables|GetLcl_DeadPlayers))))
    (if (== (Utilities|Array|Length _outactors) (LocalVariables|GetLcl_DeadPlayers))
      (Utilities|IsValid _wb_ingamehud_2
        (:Is%20Valid
          (Widget|RemovefromParent _wb_ingamehud_2)))
      (else
        (Utilities|IsValid _wb_ingamehud
          (:Is%20Valid
            (Widget|RemovefromParent _wb_ingamehud)
            (Utilities|IsValid (Variables|Default|GetWB_PlayerDiedMenu)
              (:Is%20Valid
                _)
              (:Is%20Not%20Valid
                (bind _returnvalue (UserInterface|CreateWidget "/Game/Widget/WB_PlayerDiedMenu.WB_PlayerDiedMenu_C" self))
                (Variables|Default|SetWB_PlayerDiedMenu _returnvalue)))
            (UserInterface|Viewport|AddtoViewport (Variables|Default|GetWB_PlayerDiedMenu) 0)
            (Input|SetInputModeUIOnly self 0 "DoNotLock" false)
            (Variables|Default|SetbShowMouseCursor true)))))
    (return)))

(fn SpectatorUpdateTarget
  (bind _currentspectatortarget (Variables|Default|GetCurrentSpectatorTarget))
  (Utilities|Array|Clear (Variables|Default|GetAllSpectatorTarget))
  (bind _outactors (Actor|GetAllActorsOfClass "/Game/Characters/BP_Hero_Base.BP_Hero_Base_C"))
  (for _array_element _outactors
    (Utilities|IsValid _array_element
      (:Is%20Valid
        (if (Pawn|IsPlayerControlled _array_element)
          (if (Variables|/Game/Characters/BP_Hero_Base.BP_Hero_Base_C|GetIsAlive _array_element)
            (Utilities|Array|Add (Variables|Default|GetAllSpectatorTarget) _array_element))))))
  (Utilities|IsValid _currentspectatortarget
    (:Is%20Valid
      (Variables|Default|SetSpectatorTargetIndex (Utilities|Array|FindItem (Variables|Default|GetAllSpectatorTarget) _currentspectatortarget)))
    (:Is%20Not%20Valid
      (Variables|Default|SetSpectatorTargetIndex -1))))

(fn SpectatorStartSpectateTarget
  (params (Previous :type Boolean))
  (if (> (Utilities|Array|Length (Variables|Default|GetAllSpectatorTarget)) 1)
    (if Previous
      (if (<= (Variables|Default|GetSpectatorTargetIndex) 0)
        (LocalVariables|SetLcl_NewIndex (Utilities|Array|LastIndex (Variables|Default|GetAllSpectatorTarget)))
        (else
          (LocalVariables|SetLcl_NewIndex (- (Variables|Default|GetSpectatorTargetIndex) 1))))
      (elif (== (Utilities|Array|LastIndex (Variables|Default|GetAllSpectatorTarget)) (Variables|Default|GetSpectatorTargetIndex))
        (LocalVariables|SetLcl_NewIndex 0)
        (else
          (LocalVariables|SetLcl_NewIndex (+ (Variables|Default|GetSpectatorTargetIndex) 1)))))
    (else
      (Variables|Default|SetSpectatorTargetIndex 0)))
  (bind _output_get (Variables|Default|SetSpectatorTargetIndex (LocalVariables|GetLcl_NewIndex)))
  (Utilities|IsValid (Utilities|Array|Get(acopy) (Variables|Default|GetAllSpectatorTarget) _output_get)
    (:Is%20Valid
      (bind _output_get_2 (Variables|Default|SetCurrentSpectatorTarget (Utilities|Array|Get(acopy) (Variables|Default|GetAllSpectatorTarget) _output_get)))
      (Game|Player|SetViewTargetwithBlend (Variables|/Script/Engine.ChildActorComponent|GetChildActor (Variables|/Game/Characters/BP_Hero_Base.BP_Hero_Base_C|GetSpectateTarget _output_get_2)) 0.5 "VTBlend_Linear" 0.0 false))
    (:Is%20Not%20Valid
      (Variables|Default|SetSpectatorTargetIndex -1)
      (Variables|Default|SetCurrentSpectatorTarget 0)))
  (return))

(fn SavePickedUpWeapon
  (params (WeaponRowName :type Name))
  (bind _as_sg_player_profil (Variables|Default|GetAs%20SG%20Player%20Profil))
  (bind _output_get (LocalVariables|SetLcl_Inventory (.Wpn_Inventory (Utilities|Struct|BreakS_PlayerProfil (Variables|Default|GetS%20Player%20Profile)))))
  (bind _returnvalue (Utilities|Array|AddUnique _output_get WeaponRowName))
  (if (>= _returnvalue 0)
    (bind _structout (Utilities|Struct|SetmembersinS_PlayerProfil (Variables|Default|GetS%20Player%20Profile) (LocalVariables|GetLcl_Inventory)))
    (Networking|SwitchHasAuthority
      (:Authority
        (Variables|Default|SetS%20Player%20Profile _structout))
      (:Remote
        (CallFunction|SvrSetPlayerProfil _structout)))
    (Variables|/Game/SavedData/SG_PlayerProfil.SG_PlayerProfil_C|SetPlayerProfile _as_sg_player_profil (Variables|Default|GetS%20Player%20Profile))
    (SaveGame|SaveGametoSlot _as_sg_player_profil (Variables|Default|GetSlot%20Name)))
  (return))

(fn UIToggleScoreboard
  (params (NewVisibility :type Boolean))
  (if NewVisibility
    (Utilities|IsValid (Variables|Default|GetWB_Scoreboard)
      (:Is%20Valid
        _)
      (:Is%20Not%20Valid
        (bind _returnvalue (UserInterface|CreateWidget "/Game/Widget/WB_Scoreboard.WB_Scoreboard_C" self))
        (Variables|Default|SetWB_Scoreboard _returnvalue)))
    (UserInterface|Viewport|AddtoViewport (Variables|Default|GetWB_Scoreboard) 0)
    (else
      (Utilities|IsValid (Variables|Default|GetWB_Scoreboard)
        (:Is%20Valid
          (Widget|RemovefromParent (Variables|Default|GetWB_Scoreboard)))
        (:Is%20Not%20Valid
          _))))
  (return))