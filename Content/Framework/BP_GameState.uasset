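; Game state for a shooter that replicates the match timer and player name list to each player's in-game HUD.
; Update events store new values in RepNotify variables, whose OnRep functions push them to the HUD widget on the cached player controller.
; BeginPlay caches player controller 0, which is also a RepNotify variable with an empty handler.
; Only the player names update validates the HUD widget before use.
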(event Custom|Update_HUD_PlayerNames
  (params (AllPlayerNames :type Array%20of%20Texts))
  (Variables|Default|SetAllPlayerNames AllPlayerNames))

(event Custom|UpdateHUD_MatchTimer
  (params (MatchTimeLeftSec :type Integer))
  (Variables|Default|SetMatchTimeLeftSec MatchTimeLeftSec))

(event EventBeginPlay
  (bind _asbp_shooter_player_controller (Utilities|Casting|CastToBP_Shooter_PlayerController (Game|GetPlayerController 0)))
  (Variables|Default|SetBP%20Shooter%20Player%20Controller _asbp_shooter_player_controller))

(fn ConstructionScript)

(fn OnRepBPShooterPlayerController)

(fn OnRepMatchTimeLeftSec
  (bind _bp_shooter_player_controller (Variables|Default|GetBP%20Shooter%20Player%20Controller)
    (:then
      (Default|UpdateMatchTimer (Variables|/Game/Framework/BP_Shooter_PlayerController.BP_Shooter_PlayerController_C|GetWB_IngameHUD _bp_shooter_player_controller) (Variables|Default|GetMatchTimeLeftSec)))
    (:else)))

(fn OnRepAllPlayerNames
  (bind _bp_shooter_player_controller (Variables|Default|GetBP%20Shooter%20Player%20Controller)
    (:then
      (Utilities|IsValid (Variables|/Game/Framework/BP_Shooter_PlayerController.BP_Shooter_PlayerController_C|GetWB_IngameHUD _bp_shooter_player_controller)
        (:Is%20Valid
          (Default|UpdatePlayerNames (Variables|/Game/Framework/BP_Shooter_PlayerController.BP_Shooter_PlayerController_C|GetWB_IngameHUD _bp_shooter_player_controller) (Variables|Default|GetAllPlayerNames)))))
    (:else)))