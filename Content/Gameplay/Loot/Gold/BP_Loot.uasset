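; BP_Loot is a gold pickup that grants a random amount of gold to the player who interacts with it.
; Its construction script sets the pickup row name to Gold before running the parent's construction logic.
; BeginPlay rolls the amount within a fixed range.
; On interaction, it adds that amount to the player character's TempGold and destroys itself.
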(event EventBeginPlay
  (|CallParentFunction)
  (Variables|Default|SetGold (Math|Random|RandomIntegerinRange 20 60)))

(event EventTick
  (params (DeltaSeconds :type Float%20%28single-precision%29)))

(event EventInteractwithActor
  (params (PlayerCharacter :type BP%20Hero%20Base%20Object%20Reference))
  (Variables|/Game/Characters/BP_Hero_Base.BP_Hero_Base_C|SetTempGold PlayerCharacter (+ (Variables|/Game/Characters/BP_Hero_Base.BP_Hero_Base_C|GetTempGold PlayerCharacter) (Variables|Default|GetGold)))
  (Actor|DestroyActor))

(fn ConstructionScript
  (Variables|Default|SetPickUpRowName "Gold")
  (|CallParentFunction))