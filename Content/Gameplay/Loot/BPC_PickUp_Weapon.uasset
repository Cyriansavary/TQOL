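; Weapon or ammo pickup that grants on interaction and destroys itself on success, with its data table row deciding which mesh it keeps.
; PickUp rejects ammo for unowned weapons, while new weapons are added to inventory and switched to.
; Ammo fills to max or adds loaded amounts, spilling clip overflow into stock, which is clamped to clip max.
; It also updates the active weapon's HUD and optionally has the controller save the weapon.
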(event EventInteractwithActor
  (params (PlayerCharacter :type BP%20Hero%20Base%20Object%20Reference))
  (bind _isitempickedup (CallFunction|PickUp PlayerCharacter))
  (if _isitempickedup
    (Actor|DestroyActor)))

(fn ConstructionScript
  (|CallParentFunction)
  (bind _returnvalue (Utilities|GetDataTableRow "/Game/Gameplay/Loot/PickUpInfo_Table.PickUpInfo_Table" (Variables|Default|GetPickUpRowName))
    (:then
      (bind _output_get (Variables|Default|SetIsAmmoPickUp (.IsAmmoPickUp (Utilities|Struct|BreakS_PickupInfo _returnvalue))))
      (if _output_get
        (Components|DestroyComponent (Variables|Default|GetPickUpMesh_Skeletal))
        (else
          (Components|DestroyComponent (Variables|Default|GetPickUpMesh)))))))

(fn PickUp
  (params (Player :type BP%20Hero%20Base%20Object%20Reference))
  (bind (_slottoaddweapon _isownedweapon) (Default|FindWeaponSlot Player (Variables|Default|GetWpnRowNameToAdd)))
  (LocalVariables|SetLcl_WpnInvSlot _slottoaddweapon)
  (LocalVariables|SetLcl_IsNewWeapon (not _isownedweapon))
  (if (and (LocalVariables|GetLcl_IsNewWeapon) (Variables|Default|GetIsAmmoPickUp))
    (LocalVariables|SetLcl_IsItemPickedUp false)
    (else
      (LocalVariables|SetLcl_IsItemPickedUp true)
      (bind _returnvalue (Utilities|GetDataTableRow "/Game/Weapons/WeaponInfo_Table.WeaponInfo_Table" (Variables|Default|GetWpnRowNameToAdd))
        (:then
          (if (and (LocalVariables|GetLcl_IsNewWeapon) (not (Variables|Default|GetIsAmmoPickUp)))
            (Default|SvrAddWpntoInventory Player (LocalVariables|GetLcl_WpnInvSlot) (Variables|Default|GetWpnRowNameToAdd)))
          (if (LocalVariables|GetLcl_IsNewWeapon)
            (LocalVariables|SetLcl_CurClip 0)
            (LocalVariables|SetLcl_CurClipMax (.AmmoClip (Utilities|Struct|BreakS_WeaponInfo _returnvalue)))
            (LocalVariables|SetLcl_CurStock 0)
            (LocalVariables|SetLcl_CurStockMax (.ammoStock (Utilities|Struct|BreakS_WeaponInfo _returnvalue)))
            (else
              (LocalVariables|SetLcl_CurClip (Utilities|Array|Get(acopy) (Variables|/Game/Characters/BP_Hero_Base.BP_Hero_Base_C|GetAmmoClip Player) (LocalVariables|GetLcl_WpnInvSlot)))
              (LocalVariables|SetLcl_CurClipMax (Utilities|Array|Get(acopy) (Variables|/Game/Characters/BP_Hero_Base.BP_Hero_Base_C|GetAmmoClipMax Player) (LocalVariables|GetLcl_WpnInvSlot)))
              (LocalVariables|SetLcl_CurStock (Utilities|Array|Get(acopy) (Variables|/Game/Characters/BP_Hero_Base.BP_Hero_Base_C|GetAmmoStock Player) (LocalVariables|GetLcl_WpnInvSlot)))
              (LocalVariables|SetLcl_CurStockMax (Utilities|Array|Get(acopy) (Variables|/Game/Characters/BP_Hero_Base.BP_Hero_Base_C|GetAmmoStockMax Player) (LocalVariables|GetLcl_WpnInvSlot)))))
          (if (== (Variables|Default|GetLoaded_AmmoClip) -1)
            (Utilities|Array|SetArrayElem (Variables|/Game/Characters/BP_Hero_Base.BP_Hero_Base_C|GetAmmoClip Player) (LocalVariables|GetLcl_WpnInvSlot) (LocalVariables|GetLcl_CurClipMax))
            (else
              (LocalVariables|SetLcl_ClipOverFlow (Math|Integer|Clamp(Integer) (- (+ (Variables|Default|GetLoaded_AmmoClip) (LocalVariables|GetLcl_CurClip)) (LocalVariables|GetLcl_CurClipMax)) 0 9999))
              (Utilities|Array|SetArrayElem (Variables|/Game/Characters/BP_Hero_Base.BP_Hero_Base_C|GetAmmoClip Player) (LocalVariables|GetLcl_WpnInvSlot) (Math|Integer|Clamp(Integer) (+ (Variables|Default|GetLoaded_AmmoClip) (LocalVariables|GetLcl_CurClip)) 0 (LocalVariables|GetLcl_CurClipMax)))))
          (if (== (Variables|Default|GetLoaded_AmmoClip) -1)
            (Utilities|Array|SetArrayElem (Variables|/Game/Characters/BP_Hero_Base.BP_Hero_Base_C|GetAmmoStock Player) (LocalVariables|GetLcl_WpnInvSlot) (LocalVariables|GetLcl_CurStockMax))
            (else
              (Utilities|Array|SetArrayElem (Variables|/Game/Characters/BP_Hero_Base.BP_Hero_Base_C|GetAmmoStock Player) (LocalVariables|GetLcl_WpnInvSlot) (Math|Integer|Clamp(Integer) (+ (Variables|Default|GetLoaded_AmmoStock) (LocalVariables|GetLcl_CurStock) (LocalVariables|GetLcl_ClipOverFlow)) 0 (LocalVariables|GetLcl_CurClipMax)))))
          (if (and (or (Variables|Default|GetIsAmmoPickUp) (and (not (Variables|Default|GetIsAmmoPickUp)) (not (LocalVariables|GetLcl_IsNewWeapon)))) (== (LocalVariables|GetLcl_WpnInvSlot) (Variables|/Game/Characters/BP_Hero_Base.BP_Hero_Base_C|GetActiveWeaponIndex Player)))
            (Default|ClientUpdateHUDClip Player (Utilities|Array|Get(acopy) (Variables|/Game/Characters/BP_Hero_Base.BP_Hero_Base_C|GetAmmoClip Player) (LocalVariables|GetLcl_WpnInvSlot)))
            (Default|ClientUpdateHUDStock Player (Utilities|Array|Get(acopy) (Variables|/Game/Characters/BP_Hero_Base.BP_Hero_Base_C|GetAmmoStock Player) (LocalVariables|GetLcl_WpnInvSlot))))
          (if (and (Variables|Default|GetSavedPickUpWeapon) (not (Variables|Default|GetIsAmmoPickUp)))
            (Default|ClientSavePickedUpWeapon (Variables|/Game/Characters/BP_Hero_Base.BP_Hero_Base_C|GetBP_ShooterPlayerController Player) (Variables|Default|GetWpnRowNameToAdd)))
          (if (and (LocalVariables|GetLcl_IsNewWeapon) (not (Variables|Default|GetIsAmmoPickUp)))
            (Default|MCSwitchWeapon Player (LocalVariables|GetLcl_WpnInvSlot)))))))
  (return (LocalVariables|GetLcl_IsItemPickedUp)))