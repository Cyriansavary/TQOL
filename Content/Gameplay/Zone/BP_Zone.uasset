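; BP_Zone is a shrinking zone actor that damages a hero caught outside it.
; StartZone centers the capsule on the Landscape and sizes it past the larger horizontal extent.
; Capsule overlaps cache a single hero reference and toggle its IsOutOfZone flag.
; Each ReduceZone call damages that hero if outside, shrinks the capsule radius by a Timer-based fraction and rescales the Cylinder to follow.
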(event OnComponentEndOverlap(Capsule)
  (params (OverlappedComponent :type Primitive%20Component%20Object%20Reference) (OtherActor :type Actor%20Object%20Reference) (OtherComp :type Primitive%20Component%20Object%20Reference) (OtherBodyIndex :type Integer))
  (bind _as_bp_hero_base (Variables|Default|GetAs%20BP%20Hero%20Base))
  (if (Utilities|DoesObjectImplementInterface OtherActor "/Game/Framework/Interface/BPI_Damage_Player.BPI_Damage_Player_C")
    (Variables|/Game/Characters/BP_Hero_Base.BP_Hero_Base_C|SetZone _as_bp_hero_base self)
    (Variables|/Game/Characters/BP_Hero_Base.BP_Hero_Base_C|SetIsOutOfZone _as_bp_hero_base true)))

(event OnComponentBeginOverlap(Capsule)
  (params (OverlappedComponent :type Primitive%20Component%20Object%20Reference) (OtherActor :type Actor%20Object%20Reference) (OtherComp :type Primitive%20Component%20Object%20Reference) (OtherBodyIndex :type Integer) (bFromSweep :type Boolean) (SweepResult :type Hit%20Result%20Structure%20%28by%20ref%29))
  (if (Utilities|DoesObjectImplementInterface OtherActor "/Game/Framework/Interface/BPI_Damage_Player.BPI_Damage_Player_C")
    (bind _asbp_hero_base (Utilities|Casting|CastToBP_Hero_Base OtherActor))
    (bind _output_get (Variables|Default|SetAs%20BP%20Hero%20Base _asbp_hero_base))
    (Variables|/Game/Characters/BP_Hero_Base.BP_Hero_Base_C|SetIsOutOfZone _output_get false)))

(event EventBeginPlay)

(event EventTick
  (params (DeltaSeconds :type Float%20%28single-precision%29)))

(fn ConstructionScript)

(fn StartZone
  (bind _capsule (Variables|Default|GetCapsule))
  (Variables|Default|SetStarted true)
  (Variables|/Script/Engine.PrimitiveComponent|SetbGenerateOverlapEvents (Variables|Default|GetCapsule) true)
  (bind _returnvalue (Actor|GetActorOfClass "/Script/Landscape.Landscape"))
  (bind _output_get (Variables|Default|SetLandScape _returnvalue))
  (Transformation|SetWorldLocation _capsule (.Origin (Collision|GetActorBounds _output_get false false)) false false)
  (Math|Float|CompareFloat (.x (.BoxExtent (Collision|GetActorBounds _output_get false false))) (.y (.BoxExtent (Collision|GetActorBounds _output_get false false)))
    (:>
      (Components|Capsule|SetCapsuleSize _capsule (+ (.x (.BoxExtent (Collision|GetActorBounds _output_get false false))) 2e+03) 1e+04 true :!label _label))
    (:==
      (goto _label))
    (:<
      (Components|Capsule|SetCapsuleSize _capsule (+ (.y (.BoxExtent (Collision|GetActorBounds _output_get false false))) 2e+03) 1e+04 true)))
  (return))

(fn ReduceZone
  (params (Timer :type Integer))
  (bind _capsule (Variables|Default|GetCapsule))
  (bind _as_bp_hero_base (Variables|Default|GetAs%20BP%20Hero%20Base))
  (bind _capsuleradius (Variables|/Script/Engine.CapsuleComponent|GetCapsuleRadius _capsule))
  (bind _returnvalue (/ _capsuleradius Timer))
  (bind _returnvalue_2 (- _capsuleradius _returnvalue))
  (if (Variables|Default|GetStarted)
    (if (Variables|/Game/Characters/BP_Hero_Base.BP_Hero_Base_C|GetIsOutOfZone _as_bp_hero_base)
      (Default|PlayerTakeDamage :self _as_bp_hero_base :Attacker self :Amount 5.0))
    (Components|Capsule|SetCapsuleRadius _capsule _returnvalue_2 true)
    (Transformation|SetWorldScale3D (Variables|Default|GetCylinder) (Math|Conversions|ToVector(Float) (/ _returnvalue_2 5e+01))))
  (return))